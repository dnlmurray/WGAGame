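; BP_DestrGrave is a destructible grave prop that fractures and then stops colliding as debris.
; The construction script assigns the Mesh variable to the destructible component DM and sets its cull distance.
; One second after DM fractures, its collision is switched off and a Box component takes over with query and physics collision.
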(event OnComponentFracture(DM)
  (params (HitPoint :type Vector%20%28by%20ref%29 :default "0, 0, 0") (HitDirection :type Vector%20%28by%20ref%29 :default "0, 0, 0"))
  (Utilities|FlowControl|Delay 1.0)
  (Collision|SetCollisionEnabled (Variables|Default|GetDM) "NoCollision")
  (Collision|SetCollisionEnabled (Variables|Default|GetBox) "QueryAndPhysics"))

(fn ConstructionScript
  (Class|PrimitiveComponent|SetCullDistance (Variables|Default|GetDM) 2e+03)
  (Class|DestructibleComponent|SetDestructibleMesh (Variables|Default|GetDM) (Variables|Default|GetMesh)))