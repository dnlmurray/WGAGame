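; Zombie enemy character that fights with a weapon and shows a health bar widget bound to itself.
; BeginPlay initializes the weapon from Config; Attack, intended for AI, plays a montage with weapon damage enabled for a delay scaled by attack speed.
; Input axis events also drive world-axis movement scaled by MoveSpeed.
; Dialogue participant functions supply zombie name, gender and icon, with the rest returning stub defaults.
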(event Custom|Attack
  ;[1 1 1] AI Attack
  (Class|Weapon|EnableDamageApplying (Variables|Default|GetWeapon))
  (Animation|Montage|PlayMontage (Variables|Character|GetMesh) "/Game/Characters/Enemy/Animation/Zombie_Attack_Montage.Zombie_Attack_Montage" (Variables|Default|GetEnemyAttackSpeed)
    (:then
      (Utilities|FlowControl|Delay (/ 1.3 (Variables|Default|GetEnemyAttackSpeed)))
      (Class|Weapon|DisableDamageApplying (Variables|Default|GetWeapon)))))

(event EventBeginPlay
  ;[1 1 1] Spawn a weapon in character's hand
  (Class|Weapon|Initialize (Variables|Default|GetWeapon) (Variables|Default|GetConfig))
  ;[1 1 1] HP Bar
  (bind _asenemy_health_bar (Utilities|Casting|CastToEnemyHealthBar (UserInterface|GetUserWidgetObject (Variables|Default|GetWidget))))
  (Variables|/Game/UI/EnemyHealthBar.EnemyHealthBar_C|SetEnemy _asenemy_health_bar self))

(event Input|AxisEvents|InputAxisMoveRight
  (params (AxisValue :type Float%20%28single-precision%29))
  ;[1 1 1] Movement
  (Pawn|Input|AddMovementInput "0.000000,1.000000,0.000000" (* AxisValue (Variables|Default|GetMoveSpeed)) false))

(event Input|AxisEvents|InputAxisMoveForward
  (params (AxisValue :type Float%20%28single-precision%29))
  ;[1 1 1] Movement
  (Pawn|Input|AddMovementInput "1.000000,0.000000, 0" (* AxisValue (Variables|Default|GetMoveSpeed)) false))

(fn ConstructionScript)

(fn CheckCondition
  (params (Context :type Dlg%20Context%20Object%20Reference) (ConditionName :type Name :default "None"))
  (return false))

(fn GetBoolValue
  (params (ValueName :type Name :default "None"))
  (return false))

(fn GetFloatValue
  (params (ValueName :type Name :default "None"))
  (return 0.0))

(fn GetIntValue
  (params (ValueName :type Name :default "None"))
  (return 0))

(fn GetNameValue
  (params (ValueName :type Name :default "None"))
  (return "None"))

(fn GetParticipantDisplayName
  (params (ActiveSpeaker :type Name :default "None"))
  (return "Зомби"))

(fn GetParticipantGender
  (return "Masculine"))

(fn GetParticipantIcon
  (params (ActiveSpeaker :type Name :default "None") (ActiveSpeakerState :type Name :default "None"))
  (return (Variables|Default|GetZombieMeleeSprite)))

(fn GetParticipantName
  (return "Zombie"))

(fn ModifyBoolValue
  (params (ValueName :type Name :default "None") (bNewValue :type Boolean))
  (return false))

(fn ModifyFloatValue
  (params (ValueName :type Name :default "None") (bDelta :type Boolean) (Value :type Float%20%28single-precision%29))
  (return false))

(fn ModifyIntValue
  (params (ValueName :type Name :default "None") (bDelta :type Boolean) (Value :type Integer))
  (return false))

(fn ModifyNameValue
  (params (ValueName :type Name :default "None") (NameValue :type Name :default "None"))
  (return false))

(fn OnDialogueEvent
  (params (Context :type Dlg%20Context%20Object%20Reference) (EventName :type Name :default "None"))
  (return false))