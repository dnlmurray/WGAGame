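; BP_EnemyHitVisual is a short-lived actor that leaves a blood decal near its owner, apparently as an enemy hit effect.
; On BeginPlay it shuffles its decal materials and spawns the first at a random navigable point around the owner's location.
; A dynamic material instance lets a timeline drive the Erode parameter after a delay, then the decal and actor are destroyed.
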(event EventBeginPlay
  (bind _blooddecales (Variables|Default|GetBloodDecales))
  (bind _output (Utilities|Array|Get(acopy) _blooddecales))
  (Utilities|Array|Shuffle (Variables|Default|GetBloodDecales))
  (bind _returnvalue (Rendering|Decal|SpawnDecalatLocation _output "32.000000,32.000000,64.000000" (.RandomLocation (Class|NavigationSystemV1|GetRandomPointinNavigableRadius (Transformation|GetActorLocation (Components|GetOwner)) 5e+01 0 0)) "-90.000000,0.000000,0.000000" 0.0))
  (bind _returnvalue_2 (Rendering|Material|CreateDynamicMaterialInstance _output "Erode" :!class /Script/Engine.KismetMaterialLibrary))
  (Rendering|Components|Decal|SetDecalMaterial _returnvalue _returnvalue_2)
  (Utilities|FlowControl|Delay 8.0)
  (bind _erode (Timeline|Timeline_0 PlayFromStart)
    (:Update
      (Rendering|Material|SetScalarParameterValue _returnvalue_2 "Erode" _erode :!class /Script/Engine.MaterialInstanceDynamic))
    (:Finished
      (Components|DestroyComponent _returnvalue)
      (Actor|DestroyActor))))

(fn ConstructionScript)