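; Visual-only actor for an enemy bomb explosion that leaves a poison decal on the ground.
; On BeginPlay it spawns a Niagara explosion and a downward-projected decal with randomized size and roll at its location.
; The decal and actor both last twice the bomb cooldown from Config, after which the actor destroys itself.
; A leftover debug print still runs, while a debug radius sphere is disconnected.
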(event EventBeginPlay
  (bind _returnvalue (Math|Random|RandomFloatinRange 128.0 185.0))
  (bind _returnvalue_2 (Transformation|GetActorLocation))
  (bind _config (Variables|Default|GetConfig))
  (bind _bombconfiguration (Variables|/Script/WGAGame.BombEnemyConfig|GetBombConfiguration _config))
  (bind (_damage _projectilespeed _radius _cooldown) (Utilities|Struct|BreakBombConfiguration _bombconfiguration))
  (bind _returnvalue_3 (* _cooldown 2.0))
  (Development|PrintString "Я карта Я карта ")
  (Niagara|SpawnSystematLocation "/Game/Particles/Spells/Bomb/NS_BombExplosion.NS_BombExplosion" _returnvalue_2)
  (Rendering|Decal|SpawnDecalatLocation "/Game/Materials/VFX/Decals/MI_PoisonDecal.MI_PoisonDecal" (Math|Vector|MakeVector 512.0 _returnvalue _returnvalue) _returnvalue_2 (Math|Rotator|MakeRotator (Math|Random|RandomFloatinRange -1.2e+02 1.2e+02) -9e+01 0.0) _returnvalue_3)
  (Utilities|FlowControl|Delay _returnvalue_3)
  (Actor|DestroyActor))

(fn ConstructionScript)