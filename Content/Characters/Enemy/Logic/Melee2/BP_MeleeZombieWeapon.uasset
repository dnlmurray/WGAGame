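; BP_MeleeZombieWeapon is a melee weapon Blueprint for zombie enemies that gives each weapon a random look.
; Its construction script rolls a random integer and sets the Sword static mesh component to one of five meshes: severed-limb variants, a pick or a plank.
; The roll is unseeded, so the mesh can change whenever construction reruns, and the graph changes nothing besides the mesh.
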(fn ConstructionScript
  (switch int (Math|Random|RandomIntegerinRange 0 4)
    (:0
      (Components|StaticMesh|SetStaticMesh (Variables|Default|GetSword) "/Game/Meshes/Weapon/SM_Wpn_Leg_02.SM_Wpn_Leg_02"))
    (:1
      (Components|StaticMesh|SetStaticMesh (Variables|Default|GetSword) "/Game/Meshes/Weapon/SM_Wpn_Arm.SM_Wpn_Arm"))
    (:2
      (Components|StaticMesh|SetStaticMesh (Variables|Default|GetSword) "/Game/Meshes/Weapon/SM_Wpn_Leg_01.SM_Wpn_Leg_01"))
    (:3
      (Components|StaticMesh|SetStaticMesh (Variables|Default|GetSword) "/Game/Meshes/Weapon/SM_Wpn_Pick.SM_Wpn_Pick"))
    (:4
      (Components|StaticMesh|SetStaticMesh (Variables|Default|GetSword) "/Game/Meshes/Weapon/SM_Wpn_Plank.SM_Wpn_Plank"))))