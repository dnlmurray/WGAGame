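; Ghost enemy character that attacks with thrown bombs and reports its kill to the game mode on death.
; BeginPlay sets up Health and GhostBomb from Config and links the health bar widget.
; Spawn, throw, hit and death events combine montages, fixed delays and component calls; Move Forward/Right axes also drive movement.
; Dialogue participant functions are stubs identifying it as a Zombie.
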(event Custom|LaunchBomb
  (params (TargetLocation :type Vector%20%28by%20ref%29))
  (bind _enemyattackspeed (Variables|AnimSpeed|GetEnemyAttackSpeed))
  ;[1 0 0] AI Launch Bomb
  (if (not (and (Variables|Logic|GetDeath) (Variables|Default|GetInBombThrow)))
    (Variables|Default|SetInBombThrow true)
    (Animation|PlayAnimMontage "/Game/Characters/Enemy/AnimBomb/Bomb_Throw2_Montage.Bomb_Throw2_Montage" _enemyattackspeed "None")
    (Utilities|FlowControl|Delay (/ 1.65 _enemyattackspeed))
    (Class|GhostBomb|PlaceProjectile (Variables|Default|GetGhostBomb) (Math|Transform|MakeTransform (Transformation|GetActorLocation) (Transformation|GetActorRotation)))
    (Utilities|FlowControl|Delay (.Cooldown (Utilities|Struct|BreakGhostConfiguration (Variables|/Script/WGAGame.GhostEnemyConfig|GetGhostConfiguration (Variables|Default|GetConfig)))))
    (Variables|Default|SetInBombThrow false)))

(event EventOnHitReaction
  (params (DamageAmount :type Float%20%28single-precision%29))
  ;[1 0.3845 0] HitAnim
  (Class|HealthComponent|DecreaseHealth (Variables|Default|GetHealth) DamageAmount)
  (Game|SpawnActorfromClass "/Game/Characters/Enemy/BP_EnemyHitVisual.BP_EnemyHitVisual_C" (Transformation|GetActorTransform) "Undefined" self 0)
  (Animation|PlayAnimMontage "/Game/Characters/Enemy/AnimBomb/Bomb_Impact_Montage.Bomb_Impact_Montage" (Variables|AnimSpeed|GetHitAnimSpeed) "None"))

(event EventOnDeathReaction
  (params (causer :type Actor%20Component%20Object%20Reference))
  ;[1 0.5544 0.04048] DeathAnim
  (if (not (Variables|Logic|GetDeath))
    (Variables|Logic|SetDeath true)
    (Widget|SetVisibility (UserInterface|GetUserWidgetObject (Variables|Default|GetWidget)) "Hidden")
    (bind _aswgagame_game_mode_base (Utilities|Casting|CastToWGAGameGameModeBase (Game|GetGameMode)))
    (Class|WGAGameGameModeBase|OnEnemyKill _aswgagame_game_mode_base)
    (Utilities|FlowControl|Delay 1.95)
    (Class|Enemy|OnEnemyDeath)))

(event EventOnSpawnReaction
  ;[1 0.5544 0.04048] SpawnAnim
  (Rendering|SetActorHiddenInGame false)
  (Animation|PlayAnimMontage "/Game/Characters/Enemy/AnimBomb/Bomb_Stand_Up_Montage.Bomb_Stand_Up_Montage" 1.0 "None")
  (Utilities|FlowControl|Delay 1.0))

(event EventBeginPlay
  (bind _config (Variables|Default|GetConfig))
  ;[1 1 1] Spawn a weapon in character's hand
  (Class|HealthComponent|Initialize (Variables|Default|GetHealth) _config)
  (Class|Ability|Initialize (Variables|Default|GetGhostBomb) _config)
  ;[1 1 1] HP Bar
  (bind _asenemy_health_bar (Utilities|Casting|CastToEnemyHealthBar (UserInterface|GetUserWidgetObject (Variables|Default|GetWidget))))
  (Variables|/Game/UI/EnemyHealthBar.EnemyHealthBar_C|SetEnemy _asenemy_health_bar self))

(event Input|AxisEvents|InputAxisMoveRight
  (params (AxisValue :type Float%20%28single-precision%29))
  ;[1 1 1] Movement
  (if (not (Variables|Logic|GetDeath))
    (Pawn|Input|AddMovementInput "0.000000,1.000000,0.000000" (* AxisValue (Variables|Default|GetMoveSpeed)) false)))

(event Input|AxisEvents|InputAxisMoveForward
  (params (AxisValue :type Float%20%28single-precision%29))
  ;[1 1 1] Movement
  (if (not (Variables|Logic|GetDeath))
    (Pawn|Input|AddMovementInput "1.000000,0.000000, 0" (* AxisValue (Variables|Default|GetMoveSpeed)) false)))

(fn ConstructionScript)

(fn CheckCondition
  (params (Context :type Dlg%20Context%20Object%20Reference) (ConditionName :type Name :default "None"))
  (return false))

(fn GetBoolValue
  (params (ValueName :type Name :default "None"))
  (return false))

(fn GetFloatValue
  (params (ValueName :type Name :default "None"))
  (return 0.0))

(fn GetIntValue
  (params (ValueName :type Name :default "None"))
  (return 0))

(fn GetNameValue
  (params (ValueName :type Name :default "None"))
  (return "None"))

(fn GetParticipantDisplayName
  (params (ActiveSpeaker :type Name :default "None"))
  (return "Зомби"))

(fn GetParticipantGender
  (return "Masculine"))

(fn GetParticipantIcon
  (params (ActiveSpeaker :type Name :default "None") (ActiveSpeakerState :type Name :default "None"))
  (return (Variables|Default|GetZombieMeleeSprite)))

(fn GetParticipantName
  (return "Zombie"))

(fn ModifyBoolValue
  (params (ValueName :type Name :default "None") (bNewValue :type Boolean))
  (return false))

(fn ModifyFloatValue
  (params (ValueName :type Name :default "None") (bDelta :type Boolean) (Value :type Float%20%28single-precision%29))
  (return false))

(fn ModifyIntValue
  (params (ValueName :type Name :default "None") (bDelta :type Boolean) (Value :type Integer))
  (return false))

(fn ModifyNameValue
  (params (ValueName :type Name :default "None") (NameValue :type Name :default "None"))
  (return false))

(fn OnDialogueEvent
  (params (Context :type Dlg%20Context%20Object%20Reference) (EventName :type Name :default "None"))
  (return false))