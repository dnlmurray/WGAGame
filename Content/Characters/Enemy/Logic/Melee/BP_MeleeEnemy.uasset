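; Melee skeleton enemy character that fights with a hand weapon, shows an HP bar widget and doubles as a dialogue participant named Zombie.
; Health and Weapon components initialize from Config; attacks enable weapon damage for a window scaled by attack speed.
; Hits drain health with a montage and throttled random bone-crunch sounds.
; Death hides the bar, reports the kill to the game mode and stops blocking pawns.
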(event Custom|Attack
  ;[1 0 0] AI Attack
  (if (not (Variables|Logic|GetDeath))
    (Class|Weapon|EnableDamageApplying (Variables|Default|GetWeapon))
    (Animation|Montage|PlayMontage (Variables|Character|GetMesh) "/Game/Characters/Enemy/AnimSkeleton/Skeleton_Attack_Montage.Skeleton_Attack_Montage" (Variables|AnimSpeed|GetEnemyAttackSpeed)
      (:then
        (Utilities|FlowControl|Delay (/ 1.3 (Variables|AnimSpeed|GetEnemyAttackSpeed)))
        (Class|Weapon|DisableDamageApplying (Variables|Default|GetWeapon))))))

(event Custom|HitSoundRestart
  ;[1 0.3845 0] HitAnim
  (Utilities|FlowControl|DoOnce false) ; enters at Reset
)

(event EventOnHitReaction
  (params (DamageAmount :type Float%20%28single-precision%29))
  ;[1 0.3845 0] HitAnim
  (Class|HealthComponent|DecreaseHealth (Variables|Default|GetHealth) DamageAmount)
  (if (not (Variables|Logic|GetDeath))
    (Animation|PlayAnimMontage "/Game/Characters/Enemy/AnimSkeleton/Skeleton_Impact_Montage.Skeleton_Impact_Montage" (Variables|AnimSpeed|GetHitAnimSpeed) "None")
    (Utilities|FlowControl|DoOnce false
      (:Completed
        (Utilities|SceletonImpactSound)
        (Utilities|FlowControl|Delay 1.0)
        (CallFunction|HitSoundRestart)))))

(event EventOnDeathReaction
  (params (causer :type Actor%20Component%20Object%20Reference))
  ;[1 0.5544 0.04048] DeathAnim
  (if (not (Variables|Logic|GetDeath))
    (Variables|Logic|SetDeath true)
    (Widget|SetVisibility (UserInterface|GetUserWidgetObject (Variables|Default|GetWidget)) "Hidden")
    (bind _aswgagame_game_mode_base (Utilities|Casting|CastToWGAGameGameModeBase (Game|GetGameMode)))
    (Class|WGAGameGameModeBase|OnEnemyKill _aswgagame_game_mode_base)
    (Audio|PlaySoundatLocation "/Game/Audio/enemies_damaged/bone-crushed-2.bone-crushed-2" (Transformation|GetActorLocation) "0, 0, 0" 1.0 1.0 0.0 "/Game/Audio/WGA_Medium_Attenuation.WGA_Medium_Attenuation" 0 0)
    (Utilities|FlowControl|Delay 1.0)
    (Collision|SetCollisionResponsetoChannel (Variables|Default|GetCapsuleComponent) "ECC_Pawn" "ECR_Ignore")
    (Utilities|FlowControl|Delay 0.95)
    (Class|Enemy|OnEnemyDeath)))

(event EventOnSpawnReaction
  ;[1 0.5544 0.04048] SpawnAnim
  (Rendering|SetActorHiddenInGame false)
  (Animation|PlayAnimMontage "/Game/Characters/Enemy/AnimSkeleton/Skeleton_Stand_Up_Montage.Skeleton_Stand_Up_Montage" 1.5 "None"))

(event EventBeginPlay
  (bind _config (Variables|Default|GetConfig))
  ;[1 1 1] Spawn a weapon in character's hand
  (Class|HealthComponent|Initialize (Variables|Default|GetHealth) _config)
  (Class|Weapon|Initialize (Variables|Default|GetWeapon) _config)
  ;[1 1 1] HP Bar
  (bind _asenemy_health_bar (Utilities|Casting|CastToEnemyHealthBar (UserInterface|GetUserWidgetObject (Variables|Default|GetWidget))))
  (Variables|/Game/UI/EnemyHealthBar.EnemyHealthBar_C|SetEnemy _asenemy_health_bar self))

(event Input|AxisEvents|InputAxisMoveRight
  (params (AxisValue :type Float%20%28single-precision%29))
  ;[1 1 1] Movement
  (if (not (Variables|Logic|GetDeath))
    (Pawn|Input|AddMovementInput "0.000000,1.000000,0.000000" (* AxisValue (Variables|Default|GetMoveSpeed)) false)))

(event Input|AxisEvents|InputAxisMoveForward
  (params (AxisValue :type Float%20%28single-precision%29))
  ;[1 1 1] Movement
  (if (not (Variables|Logic|GetDeath))
    (Pawn|Input|AddMovementInput "1.000000,0.000000, 0" (* AxisValue (Variables|Default|GetMoveSpeed)) false)))

(fn ConstructionScript)

(fn CheckCondition
  (params (Context :type Dlg%20Context%20Object%20Reference) (ConditionName :type Name :default "None"))
  (return false))

(fn GetBoolValue
  (params (ValueName :type Name :default "None"))
  (return false))

(fn GetFloatValue
  (params (ValueName :type Name :default "None"))
  (return 0.0))

(fn GetIntValue
  (params (ValueName :type Name :default "None"))
  (return 0))

(fn GetNameValue
  (params (ValueName :type Name :default "None"))
  (return "None"))

(fn GetParticipantDisplayName
  (params (ActiveSpeaker :type Name :default "None"))
  (return "Зомби"))

(fn GetParticipantGender
  (return "Masculine"))

(fn GetParticipantIcon
  (params (ActiveSpeaker :type Name :default "None") (ActiveSpeakerState :type Name :default "None"))
  (return (Variables|Default|GetZombieMeleeSprite)))

(fn GetParticipantName
  (return "Zombie"))

(fn ModifyBoolValue
  (params (ValueName :type Name :default "None") (bNewValue :type Boolean))
  (return false))

(fn ModifyFloatValue
  (params (ValueName :type Name :default "None") (bDelta :type Boolean) (Value :type Float%20%28single-precision%29))
  (return false))

(fn ModifyIntValue
  (params (ValueName :type Name :default "None") (bDelta :type Boolean) (Value :type Integer))
  (return false))

(fn ModifyNameValue
  (params (ValueName :type Name :default "None") (NameValue :type Name :default "None"))
  (return false))

(fn OnDialogueEvent
  (params (Context :type Dlg%20Context%20Object%20Reference) (EventName :type Name :default "None"))
  (return false))