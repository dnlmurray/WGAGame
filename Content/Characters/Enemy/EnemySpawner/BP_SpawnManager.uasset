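; Spawn manager actor that controls an EvilForce meter and triggers a one-time dialogue when the main character overlaps it.
; BeginPlay copies its range and growth rate into EvilForce.
; UpdateEvilForce refreshes the game mode's widget, then enables and resets growth or disables it based on IsActivated.
; It is also a dialogue participant supplying name, display name and gender, with conditions, values and events left as stubs.
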(event EventBeginPlay
  (bind _evilforce (Variables|Default|GetEvilForce))
  (Variables|/Script/WGAGame.EvilForce|SetMinPercent _evilforce (Variables|Default|GetMinPercent))
  (Variables|/Script/WGAGame.EvilForce|SetMaxPercent _evilforce (Variables|Default|GetMaxPercent))
  (Variables|/Script/WGAGame.EvilForce|SetEvilForceIncreasePerSecond _evilforce (Variables|Default|GetEvilForceIncreasePerSecond)))

(event Collision|EventActorBeginOverlap
  (params (OtherActor :type Actor%20Object%20Reference))
  (bind _asbp_main_character (Utilities|Casting|CastToBP_MainCharacter OtherActor))
  (if (not (Variables|Default|GetDialogueFired))
    (Default|StartDialogue _asbp_main_character (Variables|Default|GetDialogue))
    (Variables|Default|SetDialogueFired true)
    (if (not (Variables|/Game/Characters/Main_Character/BP/BP_MainCharacter.BP_MainCharacter_C|GetbStartDlgFired _asbp_main_character))
      (Utilities|FlowControl|Delay 0.2)
      (Variables|/Game/Characters/Main_Character/BP/BP_MainCharacter.BP_MainCharacter_C|SetbStartDlgFired _asbp_main_character true))))

(event EventUpdateEvilForce
  (bind _evilforce (Variables|Default|GetEvilForce))
  (bind _asbp_main_game_mode (Utilities|Casting|CastToBP_MainGameMode (Game|GetGameMode)))
  (Default|UpdateEvilForceWidget _asbp_main_game_mode)
  (if (Variables|Default|GetbIsActivated)
    (Class|EvilForce|EnableEvilForceIncreasing _evilforce)
    (Class|EvilForce|Reset _evilforce)
    (else
      (Class|EvilForce|DisableEvilForceIncreasing _evilforce))))

(fn ConstructionScript)

(fn CheckCondition
  (params (Context :type Dlg%20Context%20Object%20Reference) (ConditionName :type Name :default "None"))
  (return false))

(fn GetBoolValue
  (params (ValueName :type Name :default "None"))
  (return false))

(fn GetFloatValue
  (params (ValueName :type Name :default "None"))
  (return 0.0))

(fn GetIntValue
  (params (ValueName :type Name :default "None"))
  (return 0))

(fn GetNameValue
  (params (ValueName :type Name :default "None"))
  (return "None"))

(fn GetParticipantDisplayName
  (params (ActiveSpeaker :type Name :default "None"))
  (return (Variables|Default|GetDisplayName)))

(fn GetParticipantGender
  (return "Masculine"))

(fn GetParticipantIcon
  (params (ActiveSpeaker :type Name :default "None") (ActiveSpeakerState :type Name :default "None"))
  (return 0))

(fn GetParticipantName
  (return (Variables|Default|GetParticipantName)))

(fn ModifyBoolValue
  (params (ValueName :type Name :default "None") (bNewValue :type Boolean))
  (return false))

(fn ModifyFloatValue
  (params (ValueName :type Name :default "None") (bDelta :type Boolean) (Value :type Float%20%28single-precision%29))
  (return false))

(fn ModifyIntValue
  (params (ValueName :type Name :default "None") (bDelta :type Boolean) (Value :type Integer))
  (return false))

(fn ModifyNameValue
  (params (ValueName :type Name :default "None") (NameValue :type Name :default "None"))
  (return false))

(fn OnDialogueEvent
  (params (Context :type Dlg%20Context%20Object%20Reference) (EventName :type Name :default "None"))
  (return false))