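; BP_CheckpointManager is a checkpoint actor that plays a one-time activation effect when the main character enters its sphere outside combat.
; The overlap triggers a sound, the Angel mesh's open animation and an attached Niagara effect.
; After a short delay, Angel switches to a looping closed animation while a timeline drives the light intensity.
; The construction script sets Angel's cull distance; no save logic runs here.
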(event OnComponentBeginOverlap(Sphere)
  (params (OverlappedComponent :type Primitive%20Component%20Object%20Reference) (OtherActor :type Actor%20Object%20Reference) (OtherComp :type Primitive%20Component%20Object%20Reference) (OtherBodyIndex :type Integer) (bFromSweep :type Boolean) (SweepResult :type Hit%20Result%20Structure%20%28by%20ref%29))
  (bind _angel (Variables|Default|GetAngel))
  (bind _asbp_main_character (Utilities|Casting|CastToBP_MainCharacter OtherActor))
  (if (not (Variables|/Script/WGAGame.MainCharacter|GetbInCombat _asbp_main_character))
    (Utilities|FlowControl|DoOnce false
      (:Completed
        (Audio|PlaySoundatLocation "/Game/Audio/checkpointed/soul-saved.soul-saved" (Transformation|GetActorLocation) "0, 0, 0" 1.0 1.0 0.0 "/Game/Audio/WGA_Medium_Attenuation.WGA_Medium_Attenuation" 0 0)
        (Components|Animation|PlayAnimation _angel "/Game/Meshes/CheckPoint/SK_Checkpoint_Anim_Open.SK_Checkpoint_Anim_Open" false)
        (Niagara|SpawnSystemAttached "/Game/Particles/Environments/NS_Checkpoint.NS_Checkpoint" _angel "NS" "0, 0, 0" "0, 0, 0" "KeepRelativeOffset" true)
        (Utilities|FlowControl|Delay 1.5)
        (Components|Animation|PlayAnimation _angel "/Game/Meshes/CheckPoint/SK_Checkpoint_Anim_Closed.SK_Checkpoint_Anim_Closed" true)
        (bind _intensity (Timeline|Timeline_0 PlayFromStart)
          (:Update
            (Rendering|Components|Light|SetIntensity (Variables|Default|GetLight) (* _intensity 1.5e+04))))))))

(fn ConstructionScript
  (Class|PrimitiveComponent|SetCullDistance (Variables|Default|GetAngel) 2.5e+03))