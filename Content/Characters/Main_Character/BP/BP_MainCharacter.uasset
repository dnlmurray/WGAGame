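; Player character Blueprint with cursor-aimed movement abilities, a three-hit melee combo, dialogue participation, HUD and pause menu.
; Health, Faith, Weapon, Impulse, Exorcism and White Barrier components initialize from a shared config, most also sharing an ability state.
; Input events gate actions with boolean flags and Delay-timed montages and cooldowns.
; Kills adjust faith and health by active effects; spawning opens a dialogue that pauses the game.
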(event Custom|SelectDialogueOption
  (params (OptionIndex :type Integer))
  (bind _activecontext (Variables|Default|GetActiveContext))
  ;[1 1 1] Dialogue Option Select
  (Utilities|IsValid _activecontext
    (:Is%20Valid
      (bind _returnvalue (Class|DlgContext|ChooseOption _activecontext OptionIndex))
      (if _returnvalue
        (Default|Refresh (Variables|Default|GetDialogueWidget) (Variables|Default|GetActiveContext))
        (else
          (Default|Refresh (Variables|Default|GetDialogueWidget))
          (Game|SetGamePaused false)
          (Widget|SetVisibility (Variables|Default|GetPlayerHUD) "Visible"))))))

(event Custom|StartDialogue
  (params (Dialogue :type Dlg%20Dialogue%20Object%20Reference))
  ;[1 1 1] Start Dialogue
  (bind _returnvalue (Class|DlgManager|StartDialoguewithDefaultParticipants Dialogue))
  (Utilities|IsValid _returnvalue
    (:Is%20Valid
      (bind _output_get (Variables|Default|SetActiveContext _returnvalue))
      (Default|Refresh (Variables|Default|GetDialogueWidget) _output_get)
      (Game|SetGamePaused true)
      (Widget|SetVisibility (Variables|Default|GetPlayerHUD) "Hidden"))))

(event EventBeginPlay
  (bind _faith (Variables|Default|GetFaith))
  (bind _abilitiesconfiginst (Variables|Default|GetAbilitiesConfigInst))
  (bind _abilitiesstate (Variables|Default|GetAbilitiesState))
  ;[1 1 1] Intialize components
  (Class|FaithComponent|Initialize _faith _abilitiesconfiginst _abilitiesstate)
  (Class|HealthComponent|Initialize (Variables|Default|GetHealth) _abilitiesconfiginst _abilitiesstate)
  (Class|Weapon|Initialize (Variables|Default|GetWeapon) _abilitiesconfiginst _abilitiesstate _faith)
  (Class|Impulse|Initialize (Variables|Default|GetImpulse) _abilitiesconfiginst)
  (Class|Exorcism|Initialize (Variables|Default|GetExorcism) _abilitiesconfiginst)
  (Class|WhiteBarrier|Initialize (Variables|Default|GetWhiteBarrier) _abilitiesconfiginst _abilitiesstate)
  ;[1 1 1] Player HUD
  (bind _returnvalue (UserInterface|CreateWidget "/Game/UI/PlayerHUD.PlayerHUD_C" (Game|GetPlayerController 0)))
  (bind _output_get (Variables|Default|SetPlayerHUD _returnvalue))
  (UserInterface|Viewport|AddtoViewport _output_get 0)
  ;[1 1 1] Setting up dialogue
  (bind _returnvalue_2 (UserInterface|CreateWidget "/Game/UI/DialogueHUD.DialogueHUD_C" (Game|GetPlayerController 0)))
  (bind _output_get_2 (Variables|Default|SetDialogueWidget _returnvalue_2))
  (UserInterface|Viewport|AddtoViewport _output_get_2 0)
  (Widget|SetVisibility _output_get_2 "Collapsed")
  (Class|WGACharacter|OnSpawnReaction))

(event EventOnEnemyKill
  (bind _abilitiesstate (Variables|Default|GetAbilitiesState))
  ;[1 1 1] On enemy kill effect
  (if (or (Variables|/Script/WGAGame.AbilitiesState|GetIsUnderPureDeathEffect _abilitiesstate) (Variables|/Script/WGAGame.AbilitiesState|GetIsUnderExorcismEffect _abilitiesstate))
    (if (Variables|/Script/WGAGame.AbilitiesState|GetIsUnderPureDeathEffect (Variables|Default|GetAbilitiesState))
      (Class|FaithComponent|IncreaseFaith (Variables|Default|GetFaith) (.FaithGainPerKill (Utilities|Struct|BreakPureDeathConfiguration (Variables|/Script/WGAGame.AbilitiesConfig|GetPureDeathConfiguration (Variables|Default|GetAbilitiesConfigInst))))))
    (if (Variables|/Script/WGAGame.AbilitiesState|GetIsUnderExorcismEffect (Variables|Default|GetAbilitiesState))
      (Class|FaithComponent|IncreaseFaith (Variables|Default|GetFaith) (.FaithGainPerKill (Utilities|Struct|BreakExorcismConfiguration (Variables|/Script/WGAGame.AbilitiesConfig|GetExorcismConfiguration (Variables|Default|GetAbilitiesConfigInst))))))
    (else
      (Class|FaithComponent|DecreasePerKill (Variables|Default|GetFaith))))
  (if (Class|WhiteBarrier|IsCharacterUnderEffect (Variables|Default|GetWhiteBarrier))
    (Class|HealthComponent|IncreaseHealth (Variables|Default|GetHealth) (.HealthGainPerKill (Utilities|Struct|BreakWhiteBarrierConfiguration (Variables|/Script/WGAGame.AbilitiesConfig|GetWhiteBarrierConfiguration (Variables|Default|GetAbilitiesConfigInst))))))
  (if (Variables|/Script/WGAGame.AbilitiesState|GetIsUnderExorcismEffect (Variables|Default|GetAbilitiesState))
    (Class|HealthComponent|IncreaseHealth (Variables|Default|GetHealth) (.HealthGainPerKill (Utilities|Struct|BreakExorcismConfiguration (Variables|/Script/WGAGame.AbilitiesConfig|GetExorcismConfiguration (Variables|Default|GetAbilitiesConfigInst)))))))

(event EventOnActionStateChange
  (params (EnableFaithDecrease :type Boolean))
  (bind _faith (Variables|Default|GetFaith))
  ;[0.9875 0.993 1] Combat state change effect
  (if EnableFaithDecrease
    (Class|FaithComponent|EnableFaithDecreasing _faith)
    (else
      (Class|FaithComponent|DisableFaithDecreasing _faith))))

(event EventOnHitReaction
  (params (DamageAmount :type Float%20%28single-precision%29))
  (bind _hitanimspeed (Variables|AnimSpeed|GetHitAnimSpeed))
  ;[1 0.4595 0] HitAnim
  (Class|HealthComponent|DecreaseHealth (Variables|Default|GetHealth) DamageAmount)
  (if (not (Math|Boolean|ORBoolean (Variables|Logic|GetLeft_Hand_Attack) (Variables|Logic|GetInAction) (Variables|Logic|GetDeath) (Variables|Logic|GetInDash) (Variables|Logic|GetInWhiteBarrier)))
    (Variables|Logic|SetInAction true)
    (Animation|PlayAnimMontage "/Game/Characters/Main_Character/Animations/Sword_And_Shield_Impact_Montage.Sword_And_Shield_Impact_Montage" _hitanimspeed "None")
    (Utilities|FlowControl|Delay (/ 0.7 _hitanimspeed))
    (Variables|Logic|SetInAction false)))

(event EventOnDeathReaction
  (params (causer :type Actor%20Component%20Object%20Reference))
  ;[0.2552 0.1419 0] DeathAnim
  (Variables|Logic|SetDeath true)
  (Utilities|Casting|CastToHealthComponent causer
    (:then
      _)
    (:CastFailed
      (Utilities|Casting|CastToFaithComponent causer)))
  (Utilities|FlowControl|Delay 2.3)
  (bind _aswgagame_game_mode_base (Utilities|Casting|CastToWGAGameGameModeBase (Game|GetGameMode)))
  (Class|WGAGameGameModeBase|OnPlayerDeath _aswgagame_game_mode_base))

(event EventOnSpawnReaction
  (Development|PrintString "Player Spawned")
  (Utilities|FlowControl|Delay 0.1)
  (CallFunction|StartDialogue (Variables|Default|GetStartDlg)))

(event EventTick
  (params (DeltaSeconds :type Float%20%28single-precision%29))
  (if (Variables|Logic|GetIsCharging)
    (Development|PrintString "[PD]: Charging" true true "(R=0.000000,G=0.660000,B=1.000000,A=1.000000)" 0.1)))

(event Input|ActionEvents|InputActionLeftHand
  (params (Key :type Key%20Structure :default "None"))
  (bind _weapon (Variables|Default|GetWeapon))
  (bind _weapon_2 (Variables|Default|GetWeapon))
  ;[1 0.2703 0.2603] Combat system
  (:Pressed
    ;;[1 1 1] Click counting
    (Math|Integer|IncrementInt (Variables|Default|GetLeftClickCount)
      (:%20%20
        ;;[1 1 1] Checking are we attacking now
        (if (not (Math|Boolean|ORBoolean (Variables|Logic|GetLeft_Hand_Attack) (Variables|Logic|GetInAction) (Variables|Logic|GetDeath)))
          (Variables|Logic|SetLeft_Hand_Attack true)
          (Variables|Logic|SetInAction true)
          (Class|Weapon|EnableDamageApplying (Variables|Default|GetWeapon))
          (Utilities|FlowControl|Sequence
            (:then_0
              ;;[1 1 1] Anim of first attack
              (Animation|PlayAnimMontage "/Game/Characters/Main_Character/Animations/Standing_Melee_Attack_1_Montage.Standing_Melee_Attack_1_Montage" (Variables|AnimSpeed|GetAttackSpeed_1) "None"))
            (:then_1
              ;;[1 1 1] Delays fo previous attacks
              (Utilities|FlowControl|Delay (/ 1.06 (Variables|AnimSpeed|GetAttackSpeed_1)))
              ;;[1 1 1] Checking for 2nd attack and stoping anim of previous
              (if (and (>= (Variables|Default|GetLeftClickCount) 2) (Math|Vector|Equal(Vector) (Transformation|GetVelocity) "0, 0, 0" 5e+01))
                (Animation|StopAnimMontage "/Game/Characters/Main_Character/Animations/Standing_Melee_Attack_1_Montage.Standing_Melee_Attack_1_Montage")
                (Class|Weapon|DisableDamageApplying _weapon)
                (Class|Weapon|EnableDamageApplying _weapon)
                (Animation|PlayAnimMontage "/Game/Characters/Main_Character/Animations/Standing_Melee_Attack_2_Montage.Standing_Melee_Attack_2_Montage" (Variables|AnimSpeed|GetAttackSpeed_2) "None")
                (else
                  (Utilities|FlowControl|Delay (/ 1.2 (Variables|AnimSpeed|GetAttackSpeed_1)))
                  ;;[1 1 1] Turning off damage, attack mode and number of clicks
                  (Class|Weapon|DisableDamageApplying (Variables|Default|GetWeapon) :!label _label)
                  (Variables|Logic|SetLeft_Hand_Attack false)
                  (Variables|Logic|SetInAction false)
                  (Variables|Default|SetLeftClickCount 0))))
            (:then_2
              (Utilities|FlowControl|Delay (/ 2.0 (Variables|AnimSpeed|GetAttackSpeed_2)))
              ;;[1 1 1] Checking for 3nd attack and stoping anim of previous
              (if (>= (Variables|Default|GetLeftClickCount) 3)
                (Class|Weapon|DisableDamageApplying _weapon_2)
                (Class|Weapon|EnableDamageApplying _weapon_2)
                (Animation|PlayAnimMontage "/Game/Characters/Main_Character/Animations/Standing_Melee_Attack_3_Montage.Standing_Melee_Attack_3_Montage" (Variables|AnimSpeed|GetAttackSpeed_3) "None")
                (Utilities|FlowControl|Delay (/ 1.4 (Variables|AnimSpeed|GetAttackSpeed_3)))
                (goto _label)
                (else
                  (goto _label))))))))))

(event Input|ActionEvents|InputActionWhiteBarrier
  (params (Key :type Key%20Structure :default "None"))
  (bind _whitebarrierspeed (Variables|AnimSpeed|GetWhiteBarrierSpeed))
  ;[0.1921 0.1808 1] White Barrier placing
  (:Pressed
    (if (not (Math|Boolean|ORBoolean (Variables|Logic|GetInWhiteBarrier) (Variables|Logic|GetInAction) (Variables|Logic|GetDeath)))
      (Utilities|FlowControl|Sequence
        (:then_0
          (Variables|Logic|SetInWhiteBarrier true))
        (:then_1
          (Variables|Logic|SetInWhiteBarrierMove true))
        (:then_2
          (Variables|Logic|SetInAction true)
          (Animation|PlayAnimMontage "/Game/Characters/Main_Character/Animations/WhiteBarrier_Montage.WhiteBarrier_Montage" _whitebarrierspeed "None")
          (Utilities|FlowControl|Delay (/ 1.9 _whitebarrierspeed))
          (Class|WhiteBarrier|Place (Variables|Default|GetWhiteBarrier))
          (Variables|Logic|SetInAction false)
          (Utilities|FlowControl|Delay (/ 1.0 _whitebarrierspeed))
          (Variables|Logic|SetInWhiteBarrierMove false)
          (Utilities|FlowControl|Delay (.Cooldown (Utilities|Struct|BreakWhiteBarrierConfiguration (Variables|/Script/WGAGame.AbilitiesConfig|GetWhiteBarrierConfiguration (Variables|Default|GetAbilitiesConfigInst)))))
          (Variables|Logic|SetInWhiteBarrier false))))))

(event Input|ActionEvents|InputActionDash
  (params (Key :type Key%20Structure :default "None"))
  (bind _abilitiesconfiginst (Variables|Default|GetAbilitiesConfigInst))
  (bind _dashconfiguration (Variables|/Script/WGAGame.AbilitiesConfig|GetDashConfiguration _abilitiesconfiginst))
  (bind (_strength _cooldown) (Utilities|Struct|BreakDashConfiguration _dashconfiguration))
  ;[0.1921 0.1808 1] Dash
  (:Pressed
    (if (not (Variables|Logic|GetInDash))
      (Variables|Logic|SetInDash true)
      (bind _angle (CallFunction|CursorAngle))
      (Physics|AddImpulse (Variables|Character|GetCharacterMovement) (Math|Vector|MakeVector (.x (Class|KismetMathLibrary|CreateVectorfromYawPitch (.yaw _angle) 0.0 _strength)) (.y (Class|KismetMathLibrary|CreateVectorfromYawPitch (.yaw _angle) 0.0 _strength)) (.z (Class|KismetMathLibrary|CreateVectorfromYawPitch (.yaw _angle) 0.0 _strength))) true)
      (Utilities|FlowControl|Delay _cooldown)
      (Variables|Logic|SetInDash false))))

(event Input|ActionEvents|InputActionLeftHand
  (params (Key :type Key%20Structure :default "None"))
  ;[1 0.2703 0.2603] Combat system
  (:Pressed
    (bind _angle (CallFunction|CursorAngle))
    (if (not (Math|Boolean|ORBoolean (Variables|Logic|GetDeath) (Variables|Logic|GetInWhiteBarrierMove) (Math|Vector|NotEqual(Vector) (Transformation|GetVelocity) "0, 0, 0" 5e+01)))
      (bind _alpha (Timeline|Timeline_0 PlayFromStart)
        (:Update
          (Transformation|SetWorldRotation (Variables|Default|GetCapsuleComponent) (Math|Rotator|Lerp(Rotator) (Transformation|GetActorRotation) _angle _alpha) false false))))))

(event Input|ActionEvents|InputActionRightHand
  (params (Key :type Key%20Structure :default "None"))
  ;[0.1921 0.1808 1] Pure Death charge
  (:Pressed
    (if (not (Variables|Logic|GetIsPureDeath))
      (Variables|Logic|SetIsCharging true)
      (Utilities|FlowControl|Delay (.ChargeTime (Utilities|Struct|BreakPureDeathConfiguration (Variables|/Script/WGAGame.AbilitiesConfig|GetPureDeathConfiguration (Variables|Default|GetAbilitiesConfigInst)))))
      (if (Variables|Logic|GetIsCharging)
        (Variables|Logic|SetIsCharging false)
        (Variables|Logic|SetIsPureDeath true)
        (Variables|/Script/WGAGame.AbilitiesState|SetIsUnderPureDeathEffect (Variables|Default|GetAbilitiesState) true)
        (Variables|Logic|SetInAction true)
        (Class|Weapon|EnableDamageApplying (Variables|Default|GetWeapon))
        (Animation|PlayAnimMontage "/Game/Characters/Main_Character/Animations/Standing_Melee_Attack_1_Montage.Standing_Melee_Attack_1_Montage" (Variables|AnimSpeed|GetAttackSpeed_1) "None")
        ;;[1 1 1] Delays to attack
        (Utilities|FlowControl|Delay (/ 1.06 (Variables|AnimSpeed|GetAttackSpeed_1)))
        (Variables|/Script/WGAGame.AbilitiesState|SetIsUnderPureDeathEffect (Variables|Default|GetAbilitiesState) false)
        (Variables|Logic|SetInAction false)
        (Class|Weapon|DisableDamageApplying (Variables|Default|GetWeapon))
        (Utilities|FlowControl|Delay (.Cooldown (Utilities|Struct|BreakPureDeathConfiguration (Variables|/Script/WGAGame.AbilitiesConfig|GetPureDeathConfiguration (Variables|Default|GetAbilitiesConfigInst)))))
        (Variables|Logic|SetIsPureDeath false)))))

(event Input|ActionEvents|InputActionSkyImpulse
  (params (Key :type Key%20Structure :default "None"))
  ;[0.1921 0.1808 1] Sky Impulse place
  (:Pressed
    (if (not (Variables|Logic|GetIsSkyImpulse))
      (Variables|Logic|SetIsSkyImpulse true)
      (Class|Impulse|Place (Variables|Default|GetImpulse))
      (Utilities|FlowControl|Delay (.Cooldown (Utilities|Struct|BreakSkyImpulseConfiguration (Variables|/Script/WGAGame.AbilitiesConfig|GetSkyImpulseConfiguration (Variables|Default|GetAbilitiesConfigInst)))))
      (Variables|Logic|SetIsSkyImpulse false))))

(event Input|ActionEvents|InputActionExorcism
  (params (Key :type Key%20Structure :default "None"))
  ;[0.1921 0.1808 1] Exorcism
  (:Pressed
    (if (not (Variables|Logic|GetIsExorcism))
      (bind _output_get (Variables|Logic|SetIsExorcism true))
      (Variables|/Script/WGAGame.AbilitiesState|SetIsUnderExorcismEffect (Variables|Default|GetAbilitiesState) _output_get)
      (bind _angle (CallFunction|CursorAngle))
      (Class|Exorcism|Place (Variables|Default|GetExorcism) (Math|Vector|MakeVector (.x (Class|KismetMathLibrary|CreateVectorfromYawPitch (.yaw _angle) 0.0 1.0)) (.y (Class|KismetMathLibrary|CreateVectorfromYawPitch (.yaw _angle) 0.0 1.0)) (.z (Class|KismetMathLibrary|CreateVectorfromYawPitch (.yaw _angle) 0.0 1.0))))
      (Animation|PlayAnimMontage "/Game/Characters/Main_Character/Animations/Standing_Melee_Attack_1_Montage.Standing_Melee_Attack_1_Montage" (Variables|AnimSpeed|GetAttackSpeed_1) "None")
      ;;[1 1 1] Delays to attack
      (Utilities|FlowControl|Delay (/ 1.06 (Variables|AnimSpeed|GetAttackSpeed_1)))
      (Variables|/Script/WGAGame.AbilitiesState|SetIsUnderExorcismEffect (Variables|Default|GetAbilitiesState) false)
      (Utilities|FlowControl|Delay (.Cooldown (Utilities|Struct|BreakExorcismConfiguration (Variables|/Script/WGAGame.AbilitiesConfig|GetExorcismConfiguration (Variables|Default|GetAbilitiesConfigInst)))))
      (Variables|Logic|SetIsExorcism false))))

(event Input|AxisEvents|InputAxisMoveRight
  (params (AxisValue :type Float%20%28single-precision%29))
  ;[1 1 1] Movement
  (if (not (Math|Boolean|ORBoolean false (Variables|Logic|GetInWhiteBarrierMove) (Variables|Logic|GetDeath)))
    (Pawn|Input|AddMovementInput "0.000000,1.000000,0.000000" (* AxisValue (Variables|Default|GetMoveSpeed)) false)))

(event Input|AxisEvents|InputAxisMoveForward
  (params (AxisValue :type Float%20%28single-precision%29))
  ;[1 1 1] Movement
  (if (not (Math|Boolean|ORBoolean false (Variables|Logic|GetInWhiteBarrierMove) (Variables|Logic|GetDeath)))
    (Pawn|Input|AddMovementInput "1.000000,0.000000, 0" (* AxisValue (Variables|Default|GetMoveSpeed)) false)))

(event Input|KeyboardEvents|Escape
  (params (Key :type Key%20Structure :default "None"))
  (bind _returnvalue (Game|GetPlayerController 0))
  ;[1 1 1] Pause Menu
  (:Pressed
    (Utilities|FlowControl|FlipFlop
      (:A
        (bind _returnvalue_2 (UserInterface|CreateWidget "/Game/UI/PauseMenu.PauseMenu_C"))
        (UserInterface|Viewport|AddtoViewport _returnvalue_2 0)
        (Game|SetGamePaused true)
        (Variables|/Script/Engine.PlayerController|SetbShowMouseCursor _returnvalue true))
      (:B
        (Widget|RemovefromParent _returnvalue_2)
        (Game|SetGamePaused false)
        (Variables|/Script/Engine.PlayerController|SetbShowMouseCursor _returnvalue false)))))

(fn ConstructionScript)

(fn CursorAngle
  (bind _returnvalue (Game|GetPlayerController 0))
  (bind _returnvalue_2 (Transformation|GetActorLocation))
  (bind _hitresult (Game|Player|GetHitResultUnderCursorbyChannel _returnvalue "TraceTypeQuery1" true))
  (bind _returnvalue_3 (- (.location _hitresult) _returnvalue_2))
  (return (Math|Rotator|MakeRotfromX (Math|Vector|MakeVector (.x _returnvalue_3) (.y _returnvalue_3) 0.0))))

(fn CheckCondition
  (params (Context :type Dlg%20Context%20Object%20Reference) (ConditionName :type Name :default "None"))
  (return false))

(fn GetBoolValue
  (params (ValueName :type Name :default "None"))
  (return false))

(fn GetFloatValue
  (params (ValueName :type Name :default "None"))
  (return 0.0))

(fn GetIntValue
  (params (ValueName :type Name :default "None"))
  (return 0))

(fn GetNameValue
  (params (ValueName :type Name :default "None"))
  (return "None"))

(fn GetParticipantDisplayName
  (params (ActiveSpeaker :type Name :default "None"))
  (return " Герой"))

(fn GetParticipantGender
  (return "Masculine"))

(fn GetParticipantIcon
  (params (ActiveSpeaker :type Name :default "None") (ActiveSpeakerState :type Name :default "None"))
  (return (Variables|Default|GetPlayerSprite)))

(fn GetParticipantName
  (return "Player"))

(fn ModifyBoolValue
  (params (ValueName :type Name :default "None") (bNewValue :type Boolean))
  (return false))

(fn ModifyFloatValue
  (params (ValueName :type Name :default "None") (bDelta :type Boolean) (Value :type Float%20%28single-precision%29))
  (return false))

(fn ModifyIntValue
  (params (ValueName :type Name :default "None") (bDelta :type Boolean) (Value :type Integer))
  (return false))

(fn ModifyNameValue
  (params (ValueName :type Name :default "None") (NameValue :type Name :default "None"))
  (return false))

(fn OnDialogueEvent
  (params (Context :type Dlg%20Context%20Object%20Reference) (EventName :type Name :default "None"))
  (return false))