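; Player character for a top-down melee game, moving on world axes and turning its capsule each tick to face the mouse cursor trace.
; On BeginPlay it spawns a melee weapon on the hand socket with debug mode on and adds a health bar widget.
; Left Hand input opens a timed damage window on the weapon and sets an attack flag.
; When destroyed, it reloads the current level.
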(event EventBeginPlay
  ;[1 1 1] Spawn a weapon in character's hand
  (bind _returnvalue (Game|SpawnActorfromClass "/Game/Weapon/BP_MeleePlayerWeapon.BP_MeleePlayerWeapon_C" (Transformation|GetSocketTransform (Variables|Character|GetMesh) "WeaponSocket" "RTS_World") "Undefined" 0 0))
  (Transformation|AttachComponentToComponent _returnvalue (Variables|Character|GetMesh) "WeaponSocket" "SnapToTarget" "SnapToTarget" "SnapToTarget" true)
  (bind _output_get (Variables|Default|SetWeapon _returnvalue))
  (Class|MeleeWeapon|EnableDebugMode _output_get)
  (Variables|/Script/WGAGame.MeleeWeapon|SetWeaponOwner (Variables|Default|GetWeapon) self)
  ;[1 1 1] HP Bar
  (bind _returnvalue_2 (UserInterface|CreateWidget "/Game/UI/PlayerHealthBar.PlayerHealthBar_C" (Game|GetPlayerController 0)))
  (UserInterface|Viewport|AddtoViewport _returnvalue_2 0))

(event EventDestroyed
  ;[1 1 1] Player Death Restart
  (bind _returnvalue (Game|GetCurrentLevelName true))
  (Game|OpenLevel(byName) (Utilities|String|StringToName _returnvalue)))

(event EventTick
  (params (DeltaSeconds :type Float%20%28single-precision%29))
  (bind _returnvalue (Game|GetPlayerController 0))
  (bind _returnvalue_2 (Transformation|GetActorLocation))
  (bind _hitresult (Game|Player|GetHitResultUnderCursorbyChannel _returnvalue "TraceTypeQuery1" true))
  (bind _returnvalue_3 (- _returnvalue_2 (.location _hitresult)))
  ;[1 1 1] Rotation to mouse
  (Transformation|SetWorldRotation (Variables|Default|GetCapsuleComponent) (Math|Rotator|MakeRotator 0.0 0.0 (+ (.yaw (Math|Rotator|MakeRotationfromAxes (Math|Vector|MakeVector (.x _returnvalue_3) (.y _returnvalue_3) 0.0) "0, 0, 0" "0, 0, 0")) 9e+01)) false false))

(event Input|ActionEvents|InputActionLeftHand
  (params (Key :type Key%20Structure))
  (bind _weapon (Variables|Default|GetWeapon))
  (:Pressed
    (Class|MeleeWeapon|EnableDamageApplying _weapon)
    (Variables|Default|SetLeft_Hand_Attack true)
    (Utilities|FlowControl|Delay 0.5)
    (Variables|Default|SetLeft_Hand_Attack false)
    (Class|MeleeWeapon|DisableDamageApplying _weapon)))

(event Input|AxisEvents|InputAxisMoveRight
  (params (AxisValue :type Float%20%28single-precision%29))
  ;[1 1 1] Movement
  (Pawn|Input|AddMovementInput "0.000000,1.000000,0.000000" (* AxisValue (Variables|Default|GetMoveSpeed)) false))

(event Input|AxisEvents|InputAxisMoveForward
  (params (AxisValue :type Float%20%28single-precision%29))
  ;[1 1 1] Movement
  (Pawn|Input|AddMovementInput "1.000000,0.000000, 0" (* AxisValue (Variables|Default|GetMoveSpeed)) false))

(fn ConstructionScript)