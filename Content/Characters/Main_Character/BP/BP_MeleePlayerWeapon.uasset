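; Player melee weapon that damages enemies overlapping its hit collision.
; On BeginPlay it reads base damage from the main character's weapon attack configuration, with events to increase or reset that value.
; Separate events toggle the hit collision on and off to control when hits can land.
; Overlaps use a cast chain to call OnHitReaction on BP_MeleeEnemy, BP_MeleeEnemy2 or BP_BombEnemy with the current damage.
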(event OnComponentBeginOverlap(HitCollision)
  (params (OverlappedComponent :type Primitive%20Component%20Object%20Reference) (OtherActor :type Actor%20Object%20Reference) (OtherComp :type Primitive%20Component%20Object%20Reference) (OtherBodyIndex :type Integer) (bFromSweep :type Boolean) (SweepResult :type Hit%20Result%20Structure%20%28by%20ref%29))
  (bind _asbp_melee_enemy (Utilities|Casting|CastToBP_MeleeEnemy OtherActor)
    (:then
      (Class|WGACharacter|OnHitReaction _asbp_melee_enemy (Variables|Default|GetDamage)))
    (:CastFailed
      (bind _asbp_melee_enemy_2 (Utilities|Casting|CastToBP_MeleeEnemy2 OtherActor)
        (:then
          (Class|WGACharacter|OnHitReaction _asbp_melee_enemy_2 (Variables|Default|GetDamage)))
        (:CastFailed
          (bind _asbp_bomb_enemy (Utilities|Casting|CastToBP_BombEnemy OtherActor))
          (Class|WGACharacter|OnHitReaction _asbp_bomb_enemy (Variables|Default|GetDamage)))))))

(event Custom|EnableDamage
  (Collision|SetCollisionEnabled (Variables|Default|GetHitCollision) "QueryAndPhysics"))

(event Custom|DisableDamage
  (Collision|SetCollisionEnabled (Variables|Default|GetHitCollision) "NoCollision"))

(event Custom|ResetDamage
  (Variables|Default|SetDamage (.damage (Variables|/Script/WGAGame.BaseConfig|GetWeaponAttackConfiguration (Variables|/Script/WGAGame.MainCharacter|GetConfigInst (stale EventBeginPlay _output_get))))))

(event Custom|IncreaseDamage
  (params (Damage+ :type Float%20%28single-precision%29))
  (Variables|Default|SetDamage (+ Damage+ (Variables|Default|GetDamage))))

(event EventBeginPlay
  (bind _asbp_main_character (Utilities|Casting|CastToBP_MainCharacter (Game|GetPlayerCharacter 0)))
  (bind _output_get (Variables|Default|SetMainCharacter _asbp_main_character))
  (Variables|Default|SetDamage (.damage (Variables|/Script/WGAGame.BaseConfig|GetWeaponAttackConfiguration (Variables|/Script/WGAGame.MainCharacter|GetConfigInst _output_get)))))

(fn ConstructionScript)