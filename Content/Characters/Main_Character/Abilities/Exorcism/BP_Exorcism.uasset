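; BP_Exorcism is an actor for the main character's Exorcism ability, and its graph contains only debug visualization.
; On BeginPlay, if the configuration's Debug flag is set, it draws a box at its location and rotation, sized by configured length and width and the player capsule's half-height.
; The box lasts for the configured cooldown, after which the actor destroys itself.
; With Debug off, the graph does nothing, including no self-destruction.
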(event EventBeginPlay
  (bind _config (Variables|Default|GetConfig))
  (bind _exorcismconfiguration (Variables|/Script/WGAGame.AbilitiesConfig|GetExorcismConfiguration _config))
  (bind (_length _width _damage _faithgainperkill _healthgainperkill _cooldown _debug) (Utilities|Struct|BreakExorcismConfiguration _exorcismconfiguration))
  (if _debug
    (Rendering|Debug|DrawDebugBox (Transformation|GetActorLocation) (Math|Vector|MakeVector _length _width (Components|Capsule|GetScaledCapsuleHalfHeight (Variables|/Script/Engine.Character|GetCapsuleComponent (Game|GetPlayerCharacter 0)))) "(R=0.000000,G=0.241791,B=1.000000,A=1.000000)" (Transformation|GetActorRotation) _cooldown 1e+01)
    (Utilities|FlowControl|Delay _cooldown)
    (Actor|DestroyActor)))

(fn ConstructionScript)