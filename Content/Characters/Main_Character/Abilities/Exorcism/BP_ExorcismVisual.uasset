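; Placeholder visual actor for the main character's Exorcism ability that shows its area as a debug box.
; On BeginPlay it draws a box at its own location and rotation, with extents from the configured length and width and the first player's capsule half-height.
; Both the box and the actor last for the configured cooldown, after which the actor destroys itself.
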(event EventBeginPlay
  (bind _config (Variables|Default|GetConfig))
  (bind _exorcismconfiguration (Variables|/Script/WGAGame.MainCharacterConfig|GetExorcismConfiguration _config))
  (bind (_length _width _damage _faithcost _healthgainperkill _evilforcedecreaseperkill _cooldown) (Utilities|Struct|BreakExorcismConfiguration _exorcismconfiguration))
  (Rendering|Debug|DrawDebugBox (Transformation|GetActorLocation) (Math|Vector|MakeVector _length _width (Components|Capsule|GetScaledCapsuleHalfHeight (Variables|/Script/Engine.Character|GetCapsuleComponent (Game|GetPlayerCharacter 0)))) "(R=0.000000,G=0.241791,B=1.000000,A=1.000000)" (Transformation|GetActorRotation) _cooldown 0.0)
  (Utilities|FlowControl|Delay _cooldown)
  (Actor|DestroyActor))

(fn ConstructionScript)