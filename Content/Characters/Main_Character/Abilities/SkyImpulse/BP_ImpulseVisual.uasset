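; BP_ImpulseVisual is the visual effect actor for the main character's SkyImpulse ability.
; On BeginPlay it attaches the NS_SkyImpulse effect to the player character's left-hand socket, then after a short delay spawns two crack decals at its own location.
; Each decal gets a dynamic material instance whose Erode parameter is driven by its own timeline near the end of its lifespan, with the smaller decal lasting longer.
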(event EventBeginPlay
  (bind _returnvalue (Transformation|GetActorLocation))
  (bind _asbp_main_character (Utilities|Casting|CastToBP_MainCharacter (Game|GetPlayerCharacter 0)))
  (Niagara|SpawnSystemAttached "/Game/Particles/Spells/SkyImpulse/NS_SkyImpulse.NS_SkyImpulse" (Variables|/Script/Engine.Character|GetMesh _asbp_main_character) "S_LeftHand" "0, 0, 0" "90.000000, 0,0.000000" "KeepRelativeOffset" false)
  (Utilities|FlowControl|Delay 0.85)
  (Utilities|FlowControl|Sequence
    (:then_0
      (bind _returnvalue_2 (Rendering|Decal|SpawnDecalatLocation "/Game/Materials/VFX/SkyImpulse/MI_Cracks_01.MI_Cracks_01" "256.000000,256.000000,256.000000" _returnvalue "-90.000000,0.000000,0.000000" 4.0))
      (bind _returnvalue_3 (Rendering|Material|CreateDynamicMaterialInstance "/Game/Materials/VFX/SkyImpulse/MI_Cracks_01.MI_Cracks_01" "Erode" :!class /Script/Engine.KismetMaterialLibrary))
      (Rendering|Components|Decal|SetDecalMaterial _returnvalue_2 _returnvalue_3)
      (Utilities|FlowControl|Delay 3.0)
      (bind _erode (Timeline|Timeline_0 PlayFromStart)
        (:Update
          (Rendering|Material|SetScalarParameterValue _returnvalue_3 "Erode" _erode :!class /Script/Engine.MaterialInstanceDynamic))))
    (:then_1
      (bind _returnvalue_4 (Rendering|Decal|SpawnDecalatLocation "/Game/Materials/VFX/SkyImpulse/MI_Cracks_02.MI_Cracks_02" "128.000000,128.000000,128.000000" _returnvalue "-90.000000,0.000000,0.000000" 7.0))
      (bind _returnvalue_5 (Rendering|Material|CreateDynamicMaterialInstance "/Game/Materials/VFX/SkyImpulse/MI_Cracks_02.MI_Cracks_02" "Erode" :!class /Script/Engine.KismetMaterialLibrary))
      (Rendering|Components|Decal|SetDecalMaterial _returnvalue_4 _returnvalue_5)
      (Utilities|FlowControl|Delay 6.0)
      (bind _erode_2 (Timeline|Timeline_1 PlayFromStart)
        (:Update
          (Rendering|Material|SetScalarParameterValue _returnvalue_5 "Erode" _erode_2 :!class /Script/Engine.MaterialInstanceDynamic))))))

(fn ConstructionScript)