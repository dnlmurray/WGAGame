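; Rofler NPC spirit that starts a prayer dialogue when the main character overlaps its sphere and adjusts their exorcism abilities.
; The encounter spawns an effect, starts dialogue, and after a short delay marks prayer done.
; The player's CorrectPrayer flag then picks the paused result widget and the good or bad exorcism deltas.
; Construction sets cull distances and an optional alternate mesh and aura; dialogue participant functions are mostly stubs.
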(event OnComponentBeginOverlap(Sphere)
  (params (OverlappedComponent :type Primitive%20Component%20Object%20Reference) (OtherActor :type Actor%20Object%20Reference) (OtherComp :type Primitive%20Component%20Object%20Reference) (OtherBodyIndex :type Integer) (bFromSweep :type Boolean) (SweepResult :type Hit%20Result%20Structure%20%28by%20ref%29))
  (bind _asbp_main_character (Utilities|Casting|CastToBP_MainCharacter OtherActor))
  (if (not (Variables|Default|GetHasPrayed))
    (Niagara|SpawnSystematLocation "/Game/Particles/Chars/NS_RoflerOverlap.NS_RoflerOverlap" (+ (Transformation|GetWorldLocation (Variables|Default|GetRofler)) "0.000000,0.000000,145.000000"))
    (Default|StartDialogue _asbp_main_character (Variables|Default|GetDialogue))
    (Utilities|FlowControl|Delay 0.2)
    (Variables|Default|SetHasPrayed true)
    (Variables|/Game/Characters/Main_Character/BP/BP_MainCharacter.BP_MainCharacter_C|SetbHasPrayed _asbp_main_character true)
    (if (Variables|/Game/Characters/Main_Character/BP/BP_MainCharacter.BP_MainCharacter_C|GetbCorrectPrayer _asbp_main_character)
      (Game|SetGamePaused true)
      (bind _returnvalue (UserInterface|CreateWidget "/Game/UI/Сonsequences/Result2a.Result2a_C"))
      (UserInterface|Viewport|AddtoViewport _returnvalue 0)
      (Default|ChangeExorcismConfig _asbp_main_character (Variables|ExorcismChange|Good|GetGoodDamageDelta) (Variables|ExorcismChange|Good|GetGoodFaithCostDelta) (Variables|ExorcismChange|Good|GetGoodHPIncreaseDelta) (Variables|ExorcismChange|Good|GetGoodEvilForceDecreaseDelta) (Variables|ExorcismChange|Good|GetGoodCooldownDelta))
      (else
        (Game|SetGamePaused true)
        (bind _returnvalue_2 (UserInterface|CreateWidget "/Game/UI/Сonsequences/Result2b.Result2b_C"))
        (UserInterface|Viewport|AddtoViewport _returnvalue_2 0)
        (Default|ChangeExorcismConfig _asbp_main_character (Variables|ExorcismChange|Bad|GetBadDamageDelta) (Variables|ExorcismChange|Bad|GetBadFaithCostDelta) (Variables|ExorcismChange|Bad|GetBadHPIncreaseDelta) (Variables|ExorcismChange|Bad|GetBadEvilForceDecreaseDelta) (Variables|ExorcismChange|Bad|GetBadCooldownDelta))))))

(fn ConstructionScript
  (Class|PrimitiveComponent|SetCullDistance (Variables|Default|GetRofler) 2e+03)
  (Class|PrimitiveComponent|SetCullDistance (Variables|Default|GetAura) 2e+03)
  (if (Variables|Default|GetUse%20Rofler%202)
    (Components|StaticMesh|SetStaticMesh (Variables|Default|GetRofler) "/Game/Characters/NPC/Rofler/SM_Rofler_2.SM_Rofler_2")
    (Class|NiagaraComponent|SetAsset (Variables|Default|GetAura) "/Game/Particles/Chars/NS_Rofler2Aura.NS_Rofler2Aura")))

(fn CheckCondition
  (params (Context :type Dlg%20Context%20Object%20Reference) (ConditionName :type Name :default "None"))
  (return false))

(fn GetBoolValue
  (params (ValueName :type Name :default "None"))
  (return false))

(fn GetFloatValue
  (params (ValueName :type Name :default "None"))
  (return 0.0))

(fn GetIntValue
  (params (ValueName :type Name :default "None"))
  (return 0))

(fn GetNameValue
  (params (ValueName :type Name :default "None"))
  (return "None"))

(fn GetParticipantDisplayName
  (params (ActiveSpeaker :type Name :default "None"))
  (return "Дух"))

(fn GetParticipantGender
  (return "Masculine"))

(fn GetParticipantIcon
  (params (ActiveSpeaker :type Name :default "None") (ActiveSpeakerState :type Name :default "None"))
  (return 0))

(fn GetParticipantName
  (return (Variables|Default|GetParticipantName)))

(fn ModifyBoolValue
  (params (ValueName :type Name :default "None") (bNewValue :type Boolean))
  (return false))

(fn ModifyFloatValue
  (params (ValueName :type Name :default "None") (bDelta :type Boolean) (Value :type Float%20%28single-precision%29))
  (return false))

(fn ModifyIntValue
  (params (ValueName :type Name :default "None") (bDelta :type Boolean) (Value :type Integer))
  (return false))

(fn ModifyNameValue
  (params (ValueName :type Name :default "None") (NameValue :type Name :default "None"))
  (return false))

(fn OnDialogueEvent
  (params (Context :type Dlg%20Context%20Object%20Reference) (EventName :type Name :default "None"))
  (return false))