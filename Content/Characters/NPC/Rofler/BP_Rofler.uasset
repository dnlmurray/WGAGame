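; Spirit NPC that starts a one-time dialogue when the player enters its sphere outside combat, flagging the character as having talked to it.
; Each overlap by the player spawns a Niagara burst, and Tick shows the ASs component only while dialogue is unused and combat is off.
; The construction script sets cull distances and optionally applies the Rofler2 mesh and aura.
; Dialogue participant functions supply name and gender, with condition, value and event hooks stubbed.
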(event OnComponentBeginOverlap(Sphere)
  (params (OverlappedComponent :type Primitive%20Component%20Object%20Reference) (OtherActor :type Actor%20Object%20Reference) (OtherComp :type Primitive%20Component%20Object%20Reference) (OtherBodyIndex :type Integer) (bFromSweep :type Boolean) (SweepResult :type Hit%20Result%20Structure%20%28by%20ref%29))
  (bind _asbp_main_character (Utilities|Casting|CastToBP_MainCharacter OtherActor))
  (Niagara|SpawnSystematLocation "/Game/Particles/Chars/NS_RoflerOverlap.NS_RoflerOverlap" (+ (Transformation|GetWorldLocation (Variables|Default|GetRofler)) "0.000000,0.000000,145.000000"))
  (if (not (Variables|Default|GetbHasDialogueFired))
    (if (not (Variables|/Script/WGAGame.MainCharacter|GetbInCombat _asbp_main_character))
      (Default|StartDialogue _asbp_main_character (Variables|Default|GetDialogue))
      (Variables|Default|SetbHasDialogueFired true)
      (Variables|/Game/Characters/Main_Character/BP/BP_MainCharacter.BP_MainCharacter_C|SetbHasTalkedToRofler _asbp_main_character true))))

(event EventTick
  (params (DeltaSeconds :type Float%20%28single-precision%29))
  (bind _ass (Variables|Default|GetASs))
  (bind _asbp_main_character (Utilities|Casting|CastToBP_MainCharacter (Game|GetPlayerCharacter 0)))
  (if (and (not (Variables|Default|GetbHasDialogueFired)) (not (Variables|/Script/WGAGame.MainCharacter|GetbInCombat _asbp_main_character)))
    (Rendering|SetVisibility _ass true false)
    (else
      (Rendering|SetVisibility _ass false false))))

(fn ConstructionScript
  (Class|PrimitiveComponent|SetCullDistance (Variables|Default|GetRofler) 2e+03)
  (Class|PrimitiveComponent|SetCullDistance (Variables|Default|GetAura) 2e+03)
  (Class|PrimitiveComponent|SetCullDistance (Variables|Default|GetASs) 2e+03)
  (if (Variables|Default|GetUse%20Rofler%202)
    (Components|StaticMesh|SetStaticMesh (Variables|Default|GetRofler) "/Game/Characters/NPC/Rofler/SM_Rofler_2.SM_Rofler_2")
    (Rendering|ToggleVisibility (Variables|Default|GetASs) false)
    (Class|NiagaraComponent|SetAsset (Variables|Default|GetAura) "/Game/Particles/Chars/NS_Rofler2Aura.NS_Rofler2Aura")))

(fn CheckCondition
  (params (Context :type Dlg%20Context%20Object%20Reference) (ConditionName :type Name :default "None"))
  (return false))

(fn GetBoolValue
  (params (ValueName :type Name :default "None"))
  (return false))

(fn GetFloatValue
  (params (ValueName :type Name :default "None"))
  (return 0.0))

(fn GetIntValue
  (params (ValueName :type Name :default "None"))
  (return 0))

(fn GetNameValue
  (params (ValueName :type Name :default "None"))
  (return "None"))

(fn GetParticipantDisplayName
  (params (ActiveSpeaker :type Name :default "None"))
  (return "Дух"))

(fn GetParticipantGender
  (return "Masculine"))

(fn GetParticipantIcon
  (params (ActiveSpeaker :type Name :default "None") (ActiveSpeakerState :type Name :default "None"))
  (return 0))

(fn GetParticipantName
  (return (Variables|Default|GetParticipantName)))

(fn ModifyBoolValue
  (params (ValueName :type Name :default "None") (bNewValue :type Boolean))
  (return false))

(fn ModifyFloatValue
  (params (ValueName :type Name :default "None") (bDelta :type Boolean) (Value :type Float%20%28single-precision%29))
  (return false))

(fn ModifyIntValue
  (params (ValueName :type Name :default "None") (bDelta :type Boolean) (Value :type Integer))
  (return false))

(fn ModifyNameValue
  (params (ValueName :type Name :default "None") (NameValue :type Name :default "None"))
  (return false))

(fn OnDialogueEvent
  (params (Context :type Dlg%20Context%20Object%20Reference) (EventName :type Name :default "None"))
  (return false))