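; BP_MeleeWeaponTest is a test actor for melee weapon hit tracing, with debug mode and damage applying switched on.
; Both the construction script and BeginPlay lay out a vertical line of trace nodes along local or relative Z through SetNodes.
; Each Tick nudges the actor along X without sweeping, then runs ExecuteWeaponTrace, so the trace is exercised on a steadily moving weapon.
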(event EventTick
  (params (DeltaSeconds :type Float%20%28single-precision%29))
  (Transformation|SetActorLocation (+ (Transformation|GetActorLocation) (Math|Vector|MakeVector 2.0 0.0 0.0)) false false)
  (Class|MeleeWeapon|ExecuteWeaponTrace))

(event EventBeginPlay
  (Class|MeleeWeapon|EnableDebugMode)
  (Class|MeleeWeapon|EnableDamageApplying)
  (Class|MeleeWeapon|SetNodes (Math|Vector|MakeVector 0.0 0.0 1e+01) (Math|Vector|MakeVector 0.0 0.0 1e+02) 20))

(fn ConstructionScript
  (Class|MeleeWeapon|EnableDebugMode)
  (Class|MeleeWeapon|EnableDamageApplying)
  (Class|MeleeWeapon|SetNodes (Math|Vector|MakeVector 0.0 0.0 1e+01) (Math|Vector|MakeVector 0.0 0.0 1e+02) 20))