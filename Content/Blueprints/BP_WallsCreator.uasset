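; BP_WallsCreator is a construction-script tool that lays copies of a selectable mesh along a spline, presumably to build walls.
; It adds instanced mesh copies at mesh-length intervals, rotating each previous instance to look at the newest point so segments follow the curve.
; The final instance takes a closest-point spline rotation, though that lookup receives the instance's scale rather than its location.
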(fn ConstructionScript
  (bind _instancemesh (Variables|Default|GetInstanceMesh))
  (bind _spline (Variables|Default|GetSpline))
  (bind _mesh_length (Variables|Default|GetMesh%20Length))
  (bind _instancemesh_2 (Variables|Default|GetInstanceMesh))
  (bind _instancemesh_3 (Variables|Default|GetInstanceMesh))
  (bind _returnvalue (Components|InstancedStaticMesh|GetInstanceCount _instancemesh_3))
  (bind _returnvalue_2 (- _returnvalue 1))
  (bind _outinstancetransform (Components|InstancedStaticMesh|GetInstanceTransform _instancemesh_3 _returnvalue_2 true))
  (Components|StaticMesh|SetStaticMesh _instancemesh (Variables|Default|GetSelect%20Mesh))
  (for _index (range 0 (Math|Float|Floor (/ (Spline|GetSplineLength _spline) _mesh_length)))
    (Class|InstancedStaticMeshComponent|AddInstanceWorldSpace _instancemesh (Math|Transform|MakeTransform (Spline|GetLocationatDistanceAlongSpline _spline (* _index _mesh_length) "World") "0, 0,0.000000" "1,1,1"))
    (if (> _index 0)
      (Components|InstancedStaticMesh|UpdateInstanceTransform _instancemesh_2 (- _index 1) (Math|Transform|MakeTransform (.location (.OutInstanceTransform (Components|InstancedStaticMesh|GetInstanceTransform _instancemesh_2 (- _index 1) true))) (Math|Rotator|FindLookatRotation (.location (.OutInstanceTransform (Components|InstancedStaticMesh|GetInstanceTransform _instancemesh_2 (- _index 1) true))) (Spline|GetLocationatDistanceAlongSpline _spline (* _index _mesh_length) "World")) "1,1,1") true false false)))
  (Components|InstancedStaticMesh|UpdateInstanceTransform _instancemesh_3 _returnvalue_2 (Math|Transform|MakeTransform (.location _outinstancetransform) (Class|SplineComponent|FindRotationClosesttoWorldLocation (Variables|Default|GetSpline) (.scale _outinstancetransform) "World") "1,1,1") true false false))