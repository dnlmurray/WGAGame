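; BP_LampPost is a breakable hanging lamp that reacts to physical impacts.
; Any hit on the lamp mesh removes the light, and a hit with enough normal impulse also breaks the rope constraint and destroys the cable.
; The first hit additionally spawns glass particles, removes the firefly effect and plays a breaking sound, with the PlaySound flag preventing repeats.
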(event OnComponentHit(SM_Lamp)
  (params (HitComponent :type Primitive%20Component%20Object%20Reference) (OtherActor :type Actor%20Object%20Reference) (OtherComp :type Primitive%20Component%20Object%20Reference) (NormalImpulse :type Vector :default "0, 0, 0") (Hit :type Hit%20Result%20Structure%20%28by%20ref%29))
  (Components|DestroyComponent (Variables|Default|GetLight))
  (if (>= (Math|Float|MapRangeClamped (Math|Vector|VectorLength NormalImpulse) 5e+04 1e+06 0.0 1.0) 0.25)
    (Class|PhysicsConstraintComponent|BreakConstraint (Variables|Default|GetRope))
    (Components|DestroyComponent (Variables|Default|GetCable)))
  (if (Variables|Default|GetPlay%20Sound)
    (Niagara|SpawnSystemAttached "/Game/Particles/Environments/NS_LampGlass.NS_LampGlass" (Variables|Default|GetSM_Lamp) "None" "0, 0, 0" "0, 0, 0" "KeepRelativeOffset" false)
    (Components|DestroyComponent (Variables|Default|GetNS_Fireflies))
    (Audio|PlaySoundatLocation "/Game/Audio/SFX_GlassBreak.SFX_GlassBreak" (Transformation|GetActorLocation) "0, 0, 0" 1.0 1.0 0.0 0 0 0)
    (Variables|Default|SetPlay%20Sound false)))

(fn ConstructionScript)