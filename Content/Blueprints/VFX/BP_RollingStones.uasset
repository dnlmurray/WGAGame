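; BP_RollingStones is a one-way rockfall set piece that plays a rolling stones animation when triggered.
; Overlapping either of two triggers runs the same chain: it plays the animation once, enables collision on two "Nostepback" blockers, and destroys Trigger1.
; The construction script sets a cull distance on the smoke effect.
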(event OnComponentBeginOverlap(Trigger_1)
  (params (OverlappedComponent :type Primitive%20Component%20Object%20Reference) (OtherActor :type Actor%20Object%20Reference) (OtherComp :type Primitive%20Component%20Object%20Reference) (OtherBodyIndex :type Integer) (bFromSweep :type Boolean) (SweepResult :type Hit%20Result%20Structure%20%28by%20ref%29))
  (Components|Animation|PlayAnimation (Variables|Default|GetStones) "/Game/Meshes/Rocks/Animation/SK_RollingStones_Anim.SK_RollingStones_Anim" false)
  (Collision|SetCollisionEnabled (Variables|Default|Getnostepback) "QueryAndPhysics")
  (Collision|SetCollisionEnabled (Variables|Default|Getnostepback1) "QueryAndPhysics")
  (Components|DestroyComponent (Variables|Default|GetTrigger_1)))

(event OnComponentBeginOverlap(Trigger_2)
  (params (OverlappedComponent :type Primitive%20Component%20Object%20Reference) (OtherActor :type Actor%20Object%20Reference) (OtherComp :type Primitive%20Component%20Object%20Reference) (OtherBodyIndex :type Integer) (bFromSweep :type Boolean) (SweepResult :type Hit%20Result%20Structure%20%28by%20ref%29))
  (Components|Animation|PlayAnimation (Variables|Default|GetStones) "/Game/Meshes/Rocks/Animation/SK_RollingStones_Anim.SK_RollingStones_Anim" false)
  (Collision|SetCollisionEnabled (Variables|Default|Getnostepback) "QueryAndPhysics")
  (Collision|SetCollisionEnabled (Variables|Default|Getnostepback1) "QueryAndPhysics")
  (Components|DestroyComponent (Variables|Default|GetTrigger_1)))

(fn ConstructionScript
  (Class|PrimitiveComponent|SetCullDistance (Variables|Default|GetSmoke) 3.5e+03)
  (Class|PrimitiveComponent|SetCullDistance (Variables|Default|GetSmoke) 3.5e+03))