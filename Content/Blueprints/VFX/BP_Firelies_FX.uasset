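; BP_Firelies_FX is a VFX Blueprint that wraps a fireflies particle component, NSFireflies, and exposes its look as Blueprint variables.
; The Construction Script pushes radius, vortex strength, spawn count, color and size into the effect's user parameters.
; SphereRadius drives the parameter named "Sphere Location", and Color is passed as a Vec3.
; The file contains no runtime event logic.
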(fn ConstructionScript
  (bind _ns_fireflies (Variables|Default|GetNS_Fireflies))
  (Utilities|FlowControl|Sequence
    (:then_0
      (Niagara|SetNiagaraVariable(Float) _ns_fireflies "Sphere Location" (Variables|Niagara|GetSphere%20Radius)))
    (:then_1
      (Niagara|SetNiagaraVariable(Float) _ns_fireflies "Vortex Strength" (Variables|Niagara|GetVortex%20Strength)))
    (:then_2
      (Class|NiagaraComponent|SetVariableInt _ns_fireflies "Spawn Count" (Variables|Niagara|GetSpawn%20Count)))
    (:then_3
      (Niagara|SetNiagaraVariable(Vector3) _ns_fireflies "Color" (Variables|Niagara|GetColor)))
    (:then_4
      (Niagara|SetNiagaraVariable(Float) _ns_fireflies "Size" (Variables|Niagara|GetSize)))))