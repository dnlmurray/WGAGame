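; BP_Flies_FX is a placeable effect Blueprint that wraps a Niagara system of flies.
; The construction script sets a cull distance on the Niagara component, then passes the radius, vortex strength and spawn count variables into its user parameters.
; The radius feeds a float parameter named "Sphere Location", and the "DF Influence" setter is left unconnected, so it never runs.
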(fn ConstructionScript
  (bind _ns_flies (Variables|Default|GetNS_Flies))
  (Class|PrimitiveComponent|SetCullDistance (Variables|Default|GetNS_Flies) 1.5e+03)
  (Utilities|FlowControl|Sequence
    (:then_0
      (Niagara|SetNiagaraVariable(Float) _ns_flies "Sphere Location" (Variables|Niagara|GetSphere%20Radius)))
    (:then_1
      (Niagara|SetNiagaraVariable(Float) _ns_flies "Vortex Strength" (Variables|Niagara|GetVortex%20Strength)))
    (:then_2
      (Class|NiagaraComponent|SetVariableInt _ns_flies "Spawn Count" (Variables|Niagara|GetSpawn%20Count)))))