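; BP_MainGameMode is the game mode that manages the Evil Force HUD widget for the spawn manager.
; It creates WB_EvilForce at BeginPlay, and UpdateEvilForceWidget hands it the BP_SpawnManager reference, then shows or removes it based on whether that manager is activated.
; GetEvilForcePercent exposes the spawn manager's Evil Force percentage.
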(event Custom|UpdateEvilForceWidget
  (bind _evilforcewidget (Variables|Default|GetEvilForceWidget))
  (bind _asbp_spawn_manager (Utilities|Casting|CastToBP_SpawnManager (Variables|Default|GetSpawnManager)))
  (Variables|/Game/UI/WB_EvilForce.WB_EvilForce_C|SetSpawnManager (Variables|Default|GetEvilForceWidget) _asbp_spawn_manager)
  (if (Variables|/Script/WGAGame.SpawnManager|GetbIsActivated (Variables|Default|GetSpawnManager))
    (UserInterface|Viewport|AddtoViewport _evilforcewidget 0)
    (else
      (Widget|RemovefromParent _evilforcewidget))))

(event EventBeginPlay
  (bind _returnvalue (UserInterface|CreateWidget "/Game/UI/WB_EvilForce.WB_EvilForce_C"))
  (Variables|Default|SetEvilForceWidget _returnvalue))

(fn ConstructionScript)

(fn GetEvilForcePercent
  (bind _asbp_spawn_manager (Utilities|Casting|CastToBP_SpawnManager (Variables|Default|GetSpawnManager)))
  (return (Variables|/Script/WGAGame.EvilForce|GetPercent (Variables|/Game/Characters/Enemy/EnemySpawner/BP_SpawnManager.BP_SpawnManager_C|GetEvilForce _asbp_spawn_manager))))