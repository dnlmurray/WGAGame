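; BP_GravesCreator is a construction-script placement tool that scatters copies of a mesh, presumably graves going by its name, in a randomized grid.
; It adds an instanced static mesh component with the chosen Mesh, then loops over Rows and Columns to add instances.
; Each instance gets position jitter proportional to the grid spacing, random yaw and random uniform scale around 1, with no fixed seed.
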(fn ConstructionScript
  (bind _distance_between (Variables|Main|GetDistance%20Between))
  (bind _randomize_distance (Variables|Random|GetRandomize%20Distance))
  (bind _instancedmesh (Variables|Default|GetInstancedMesh))
  (bind _randomize_scale (Variables|Random|GetRandomize%20Scale))
  (bind _randomize_rotation (Variables|Random|GetRandomize%20Rotation))
  (bind _distance_between_2 (Variables|Main|GetDistance%20Between))
  (bind _randomize_distance_2 (Variables|Random|GetRandomize%20Distance))
  (bind _returnvalue (Components|StaticMesh|SetStaticMesh _instancedmesh (Variables|Main|GetMesh)))
  (AddComponent|AddInstancedStaticMeshComponent _returnvalue)
  (for _index (range 0 (Variables|Main|GetRows))
    (for _index_2 (range 0 (Variables|Main|GetColumns))
      (Components|InstancedStaticMesh|AddInstance _instancedmesh (Math|Transform|MakeTransform (Math|Vector|MakeVector (+ (* _index _distance_between) (* _distance_between (Math|Random|RandomFloatinRange (* _randomize_distance -1.0) _randomize_distance))) (+ (* _index_2 _distance_between_2) (* _distance_between_2 (Math|Random|RandomFloatinRange (* _randomize_distance_2 -1.0) _randomize_distance_2))) 0.0) (Math|Rotator|MakeRotator 0.0 0.0 (Math|Random|RandomFloatinRange (* _randomize_rotation -1.0) _randomize_rotation)) (Math|Conversions|ToVector(Float) (+ (Math|Random|RandomFloatinRange (* _randomize_scale -1.0) _randomize_scale) 1.0)))))))