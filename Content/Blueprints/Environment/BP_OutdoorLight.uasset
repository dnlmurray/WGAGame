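; BP_OutdoorLight stages lighting and weather changes as overlaps hit four one-shot trigger volumes.
; Timelines animate the Direct light's intensity at every trigger, and MPC_WeatherControls wind at the first three.
; Trigger 1 also animates puddle size, Trigger 2 the player character's rain spawn rate, and Trigger 3 fog color.
; Chained timelines start from the preceding one's Update, so they restart until that one finishes.
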(event OnComponentBeginOverlap(Trigger_1)
  (params (OverlappedComponent :type Primitive%20Component%20Object%20Reference) (OtherActor :type Actor%20Object%20Reference) (OtherComp :type Primitive%20Component%20Object%20Reference) (OtherBodyIndex :type Integer) (bFromSweep :type Boolean) (SweepResult :type Hit%20Result%20Structure%20%28by%20ref%29))
  (Utilities|FlowControl|DoOnce false
    (:Completed
      (bind _intensity (Timeline|Timeline_0 PlayFromStart)
        (:Update
          (Rendering|Components|Light|SetIntensity (Variables|Default|GetDirect) _intensity)
          (bind _intensity_2 (Timeline|Timeline_2 PlayFromStart)
            (:Update
              (Rendering|Material|SetScalarParameterValue "/Game/Materials/MPC_WeatherControls.MPC_WeatherControls" "Wind Intensity" _intensity_2 :!class /Script/Engine.KismetMaterialLibrary)
              (bind _puddles (Timeline|Timeline_7 PlayFromStart)
                (:Update
                  (Rendering|Material|SetScalarParameterValue "/Game/Materials/MPC_WeatherControls.MPC_WeatherControls" "Puddles Size" _puddles :!class /Script/Engine.KismetMaterialLibrary))))))))))

(event OnComponentBeginOverlap(Trigger_2)
  (params (OverlappedComponent :type Primitive%20Component%20Object%20Reference) (OtherActor :type Actor%20Object%20Reference) (OtherComp :type Primitive%20Component%20Object%20Reference) (OtherBodyIndex :type Integer) (bFromSweep :type Boolean) (SweepResult :type Hit%20Result%20Structure%20%28by%20ref%29))
  (Utilities|FlowControl|DoOnce false
    (:Completed
      (bind _intensity (Timeline|Timeline_1 PlayFromStart)
        (:Update
          (Rendering|Components|Light|SetIntensity (Variables|Default|GetDirect) _intensity)
          (bind _intensity_2 (Timeline|Timeline_5 PlayFromStart)
            (:Update
              (Rendering|Material|SetScalarParameterValue "/Game/Materials/MPC_WeatherControls.MPC_WeatherControls" "Wind Intensity" _intensity_2 :!class /Script/Engine.KismetMaterialLibrary)
              (bind _asbp_main_character (Utilities|Casting|CastToBP_MainCharacter (Game|GetPlayerCharacter 0)))
              (bind _rain (Timeline|rain PlayFromStart)
                (:Update
                  (Niagara|SetNiagaraVariable(Float) (Variables|/Game/Characters/Main_Character/BP/BP_MainCharacter.BP_MainCharacter_C|GetRain _asbp_main_character) "Spawn Rate" (* _rain 1e+03)))))))))))

(event OnComponentBeginOverlap(Trigger_3)
  (params (OverlappedComponent :type Primitive%20Component%20Object%20Reference) (OtherActor :type Actor%20Object%20Reference) (OtherComp :type Primitive%20Component%20Object%20Reference) (OtherBodyIndex :type Integer) (bFromSweep :type Boolean) (SweepResult :type Hit%20Result%20Structure%20%28by%20ref%29))
  (Utilities|FlowControl|DoOnce false
    (:Completed
      (bind _color (Timeline|Timeline_8 PlayFromStart)
        (:Update
          (Rendering|Material|SetVectorParameterValue "/Game/Materials/MPC_WeatherControls.MPC_WeatherControls" "Fog Color" _color :!class /Script/Engine.KismetMaterialLibrary)
          (bind _intensity (Timeline|Timeline_3 PlayFromStart)
            (:Update
              (Rendering|Components|Light|SetIntensity (Variables|Default|GetDirect) _intensity)
              (bind _intensity_2 (Timeline|Timeline_6 PlayFromStart)
                (:Update
                  (Rendering|Material|SetScalarParameterValue "/Game/Materials/MPC_WeatherControls.MPC_WeatherControls" "Wind Intensity" _intensity_2 :!class /Script/Engine.KismetMaterialLibrary))))))))))

(event OnComponentBeginOverlap(Trigger_4)
  (params (OverlappedComponent :type Primitive%20Component%20Object%20Reference) (OtherActor :type Actor%20Object%20Reference) (OtherComp :type Primitive%20Component%20Object%20Reference) (OtherBodyIndex :type Integer) (bFromSweep :type Boolean) (SweepResult :type Hit%20Result%20Structure%20%28by%20ref%29))
  (Utilities|FlowControl|DoOnce false
    (:Completed
      (bind _intensity (Timeline|Timeline_4 PlayFromStart)
        (:Update
          (Rendering|Components|Light|SetIntensity (Variables|Default|GetDirect) _intensity))))))

(fn ConstructionScript)