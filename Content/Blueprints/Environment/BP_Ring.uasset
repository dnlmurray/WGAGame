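; BP_Ring is a quest pickup in the ghost girl storyline that also serves as the "Ring" dialogue participant.
; Tick polls the player's quest flags and shows the ASs component only after talking to the ghost girl and before finding the ring.
; Overlapping its sphere in that state starts FoundRingDialogue on the main character.
; Dialogue interface functions other than the participant name are stubs returning defaults.
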(event OnComponentBeginOverlap(Sphere)
  (params (OverlappedComponent :type Primitive%20Component%20Object%20Reference) (OtherActor :type Actor%20Object%20Reference) (OtherComp :type Primitive%20Component%20Object%20Reference) (OtherBodyIndex :type Integer) (bFromSweep :type Boolean) (SweepResult :type Hit%20Result%20Structure%20%28by%20ref%29))
  (bind _asbp_main_character (Utilities|Casting|CastToBP_MainCharacter OtherActor))
  (if (and (Variables|/Game/Characters/Main_Character/BP/BP_MainCharacter.BP_MainCharacter_C|GetbHasTalkedToGhostGirl _asbp_main_character) (not (Variables|/Game/Characters/Main_Character/BP/BP_MainCharacter.BP_MainCharacter_C|GetbHasFoundRing _asbp_main_character)))
    (Default|StartDialogue _asbp_main_character "/Game/Characters/Dialogues/FoundRingDialogue.FoundRingDialogue")))

(event EventBeginPlay)

(event Collision|EventActorBeginOverlap
  (params (OtherActor :type Actor%20Object%20Reference)))

(event EventTick
  (params (DeltaSeconds :type Float%20%28single-precision%29))
  (bind _ass (Variables|Default|GetASs))
  (bind _asbp_main_character (Utilities|Casting|CastToBP_MainCharacter (Game|GetPlayerCharacter 0)))
  (if (and (Variables|/Game/Characters/Main_Character/BP/BP_MainCharacter.BP_MainCharacter_C|GetbHasTalkedToGhostGirl _asbp_main_character) (not (Variables|/Game/Characters/Main_Character/BP/BP_MainCharacter.BP_MainCharacter_C|GetbHasFoundRing _asbp_main_character)))
    (Rendering|SetVisibility _ass true false)
    (else
      (Rendering|SetVisibility _ass false false))))

(fn ConstructionScript
  (Class|PrimitiveComponent|SetCullDistance (Variables|Default|GetASs) 2e+03)
  (Rendering|ToggleVisibility (Variables|Default|GetASs) false))

(fn CheckCondition
  (params (Context :type Dlg%20Context%20Object%20Reference) (ConditionName :type Name :default "None"))
  (return false))

(fn GetBoolValue
  (params (ValueName :type Name :default "None"))
  (return false))

(fn GetFloatValue
  (params (ValueName :type Name :default "None"))
  (return 0.0))

(fn GetIntValue
  (params (ValueName :type Name :default "None"))
  (return 0))

(fn GetNameValue
  (params (ValueName :type Name :default "None"))
  (return "None"))

(fn GetParticipantDisplayName
  (params (ActiveSpeaker :type Name :default "None"))
  (return ""))

(fn GetParticipantGender
  (return "Masculine"))

(fn GetParticipantIcon
  (params (ActiveSpeaker :type Name :default "None") (ActiveSpeakerState :type Name :default "None"))
  (return 0))

(fn GetParticipantName
  (return "Ring"))

(fn ModifyBoolValue
  (params (ValueName :type Name :default "None") (bNewValue :type Boolean))
  (return false))

(fn ModifyFloatValue
  (params (ValueName :type Name :default "None") (bDelta :type Boolean) (Value :type Float%20%28single-precision%29))
  (return false))

(fn ModifyIntValue
  (params (ValueName :type Name :default "None") (bDelta :type Boolean) (Value :type Integer))
  (return false))

(fn ModifyNameValue
  (params (ValueName :type Name :default "None") (NameValue :type Name :default "None"))
  (return false))

(fn OnDialogueEvent
  (params (Context :type Dlg%20Context%20Object%20Reference) (EventName :type Name :default "None"))
  (return false))