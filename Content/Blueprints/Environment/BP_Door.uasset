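; Gravekeeper's door that acts as a dialogue participant and opens once the player character's HasOpenedGravekeeperDoor flag is set.
; Trigger overlap outside combat either starts the Gravekeeper dialogue or, through a DoOnce, plays the door animation and swaps closed collision for open.
; Tick shows an attention sign while NeedToSpeak is true and the player is out of combat.
; Dialogue interface functions supply only the speaker's identity; conditions, values and events are stubs.
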(event OnComponentBeginOverlap(Trigger)
  (params (OverlappedComponent :type Primitive%20Component%20Object%20Reference) (OtherActor :type Actor%20Object%20Reference) (OtherComp :type Primitive%20Component%20Object%20Reference) (OtherBodyIndex :type Integer) (bFromSweep :type Boolean) (SweepResult :type Hit%20Result%20Structure%20%28by%20ref%29))
  (bind _asbp_main_character (Utilities|Casting|CastToBP_MainCharacter (Game|GetPlayerCharacter 0)))
  (if (not (Variables|/Script/WGAGame.MainCharacter|GetbInCombat _asbp_main_character))
    (if (Variables|/Game/Characters/Main_Character/BP/BP_MainCharacter.BP_MainCharacter_C|GetHasOpenedGravekeeperDoor _asbp_main_character)
      (Utilities|FlowControl|DoOnce false :!label _label
        (:Completed
          (Components|Animation|PlayAnimation (Variables|Default|GetDoor) "/Game/Meshes/Artificial/Buildings/Door/SK_Door_Anim.SK_Door_Anim" false)
          (Collision|SetCollisionEnabled (Variables|Default|GetClosed%20Collision) "NoCollision")
          (Collision|SetCollisionEnabled (Variables|Default|GetOpen%20Collision) "QueryAndPhysics")))
      (else
        (Default|StartDialogue _asbp_main_character "/Game/Characters/Dialogues/GravekeeperDialogue.GravekeeperDialogue")
        (if (Variables|/Game/Characters/Main_Character/BP/BP_MainCharacter.BP_MainCharacter_C|GetHasOpenedGravekeeperDoor _asbp_main_character)
          (goto _label Reset))))))

(event EventTick
  (params (DeltaSeconds :type Float%20%28single-precision%29))
  (bind _attentionsign (Variables|Default|GetAttentionSign))
  (bind _asbp_main_character (Utilities|Casting|CastToBP_MainCharacter (Game|GetPlayerCharacter 0)))
  (if (and (not (Variables|/Script/WGAGame.MainCharacter|GetbInCombat _asbp_main_character)) (Variables|Default|GetNeedToSpeak))
    (Rendering|SetVisibility _attentionsign true false)
    (else
      (Rendering|SetVisibility _attentionsign false false))))

(fn ConstructionScript
  (Class|PrimitiveComponent|SetCullDistance (Variables|Default|GetDoor) 2e+03))

(fn CheckCondition
  (params (Context :type Dlg%20Context%20Object%20Reference) (ConditionName :type Name :default "None"))
  (return false))

(fn GetBoolValue
  (params (ValueName :type Name :default "None"))
  (return false))

(fn GetFloatValue
  (params (ValueName :type Name :default "None"))
  (return 0.0))

(fn GetIntValue
  (params (ValueName :type Name :default "None"))
  (return 0))

(fn GetNameValue
  (params (ValueName :type Name :default "None"))
  (return "None"))

(fn GetParticipantDisplayName
  (params (ActiveSpeaker :type Name :default "None"))
  (return "Гробовщик"))

(fn GetParticipantGender
  (return "Masculine"))

(fn GetParticipantIcon
  (params (ActiveSpeaker :type Name :default "None") (ActiveSpeakerState :type Name :default "None"))
  (return 0))

(fn GetParticipantName
  (return "Gravekeeper"))

(fn ModifyBoolValue
  (params (ValueName :type Name :default "None") (bNewValue :type Boolean))
  (return false))

(fn ModifyFloatValue
  (params (ValueName :type Name :default "None") (bDelta :type Boolean) (Value :type Float%20%28single-precision%29))
  (return false))

(fn ModifyIntValue
  (params (ValueName :type Name :default "None") (bDelta :type Boolean) (Value :type Integer))
  (return false))

(fn ModifyNameValue
  (params (ValueName :type Name :default "None") (NameValue :type Name :default "None"))
  (return false))

(fn OnDialogueEvent
  (params (Context :type Dlg%20Context%20Object%20Reference) (EventName :type Name :default "None"))
  (return false))