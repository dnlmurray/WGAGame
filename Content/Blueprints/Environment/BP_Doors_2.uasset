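; Door actor that opens for the main character only when out of combat and after they have talked to Rofler.
; An Open overlap plays the skeletal opening animation and sound and disables the closed-door collision.
; A Close overlap, with no actor check, plays closing effects, restores that collision and disables both open-door collisions.
; Each direction fires once until its reset event runs; construction sets the mesh cull distance.
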(event OnComponentBeginOverlap(Open)
  (params (OverlappedComponent :type Primitive%20Component%20Object%20Reference) (OtherActor :type Actor%20Object%20Reference) (OtherComp :type Primitive%20Component%20Object%20Reference) (OtherBodyIndex :type Integer) (bFromSweep :type Boolean) (SweepResult :type Hit%20Result%20Structure%20%28by%20ref%29))
  (bind _asbp_main_character (Utilities|Casting|CastToBP_MainCharacter OtherActor))
  (if (not (Variables|/Script/WGAGame.MainCharacter|GetbInCombat _asbp_main_character))
    (if (Variables|/Game/Characters/Main_Character/BP/BP_MainCharacter.BP_MainCharacter_C|GetbHasTalkedToRofler _asbp_main_character)
      (Utilities|FlowControl|DoOnce false
        (:Completed
          (Components|Animation|PlayAnimation (Variables|Default|GetSK_Doors) "/Game/Meshes/Artificial/Walls/Doors/SK_Doors_Open_Anim.SK_Doors_Open_Anim" false)
          (Audio|SpawnSoundatLocation "/Game/Audio/environment/DoorsOpen.DoorsOpen" (Transformation|GetActorLocation) "0, 0, 0" 1.5 1.0 2.5 "/Game/Audio/WGA_Medium_Attenuation.WGA_Medium_Attenuation" 0)
          (Collision|SetCollisionEnabled (Variables|Default|GetCollisionClosed) "NoCollision"))))))

(event OnComponentBeginOverlap(Close)
  (params (OverlappedComponent :type Primitive%20Component%20Object%20Reference) (OtherActor :type Actor%20Object%20Reference) (OtherComp :type Primitive%20Component%20Object%20Reference) (OtherBodyIndex :type Integer) (bFromSweep :type Boolean) (SweepResult :type Hit%20Result%20Structure%20%28by%20ref%29))
  (Utilities|FlowControl|DoOnce false
    (:Completed
      (Components|Animation|PlayAnimation (Variables|Default|GetSK_Doors) "/Game/Meshes/Artificial/Walls/Doors/SK_Doors_Close.SK_Doors_Close" false)
      (Audio|SpawnSoundatLocation "/Game/Audio/environment/DoorsClosed.DoorsClosed" (Transformation|GetActorLocation) "0, 0, 0" 1.5 1.0 2.0 "/Game/Audio/WGA_Medium_Attenuation.WGA_Medium_Attenuation" 0)
      (Collision|SetCollisionEnabled (Variables|Default|GetCollisionClosed) "QueryAndPhysics")
      (Collision|SetCollisionEnabled (Variables|Default|GetCollisionOpen_1) "NoCollision")
      (Collision|SetCollisionEnabled (Variables|Default|GetCollisionOpen_2) "NoCollision"))))

(event Custom|RestDoorsOpen
  (Utilities|FlowControl|DoOnce false) ; enters at Reset
)

(event Custom|RestDoorsClose
  (Utilities|FlowControl|DoOnce false) ; enters at Reset
)

(fn ConstructionScript
  (Class|PrimitiveComponent|SetCullDistance (Variables|Default|GetSK_Doors) 2.2e+03))