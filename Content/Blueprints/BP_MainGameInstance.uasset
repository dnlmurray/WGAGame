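; Game instance that acts as the central UI manager for main menu, pause, options, death, loading, tutorial, hint and result screens.
; Each event lazily creates and caches its widget, adds it to the viewport, and where needed switches input mode or pauses the game.
; It also opens levels for game start and return to menu.
; On death, BackToCheckpoint asks BP_MainGameMode to load a reached checkpoint, otherwise restarts Level1_rebuild.
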(event Custom|Show%20Main%20Menu
  (bind _returnvalue (Game|GetPlayerController 0))
  ;[1 1 1] Main Menu
  (Variables|/Script/Engine.PlayerController|SetbShowMouseCursor (Game|GetPlayerController 0) true)
  ;;[1 1 1] Показываем главное меню
  (Utilities|IsValid (Variables|Widgets|GetMainMenuWidget)
    (:Is%20Valid
      _)
    (:Is%20Not%20Valid
      (bind _returnvalue_2 (UserInterface|CreateWidget "/Game/UI/WB_MainMenu.WB_MainMenu_C" _returnvalue))
      (bind _output_get (Variables|Widgets|SetMainMenuWidget _returnvalue_2))))
  (UserInterface|Viewport|AddtoViewport _output_get 0)
  (Input|SetInputModeUIOnly _returnvalue 0 "LockInFullscreen")
  (Variables|Logic|SetInMenu true))

(event Custom|ShowLoadingScreen
  ;[1 1 1] Main Menu
  ;;[1 1 1] Show Loading Screen
  (Utilities|IsValid (Variables|Widgets|GetLoadingScreenWidget)
    (:Is%20Valid
      _)
    (:Is%20Not%20Valid
      (bind _returnvalue (UserInterface|CreateWidget "/Game/UI/WB_LoadingScreen.WB_LoadingScreen_C" (Game|GetPlayerController 0)))
      (bind _output_get (Variables|Widgets|SetLoadingScreenWidget _returnvalue))))
  (UserInterface|Viewport|AddtoViewport _output_get 0))

(event Custom|DeathToNewGame
  ;[1 1 1] Death Screen
  (Widget|RemovefromParent (Variables|Widgets|GetDeathScreenWidget))
  (Game|OpenLevel(byName) "Level1_rebuild")
  (Input|SetInputModeGameandUI (Game|GetPlayerController 0) 0 "DoNotLock" true))

(event Custom|StartHint1_1
  ;[1 1 1] Hints
  ;;[1 1 1] Hint 1
  ;;;[1 1 1] StartHint1
  (Utilities|IsValid (Variables|Hints|GetHint1_1)
    (:Is%20Valid
      _)
    (:Is%20Not%20Valid
      (bind _returnvalue (UserInterface|CreateWidget "/Game/UI/Hints/Hint1_1.Hint1_1_C"))
      (bind _output_get (Variables|Hints|SetHint1_1 _returnvalue))))
  (UserInterface|Viewport|AddtoViewport _output_get 0)
  (Input|SetInputModeUIOnly (Game|GetPlayerController 0) 0 "LockInFullscreen"))

(event Custom|StartHint1_2
  ;[1 1 1] Hints
  ;;[1 1 1] Hint 1
  ;;;[1 1 1] Start Hint 1_2
  (Utilities|IsValid (Variables|Hints|GetHint1_2)
    (:Is%20Valid
      _)
    (:Is%20Not%20Valid
      (bind _returnvalue (UserInterface|CreateWidget "/Game/UI/Hints/Hint1_2.Hint1_2_C"))
      (bind _output_get (Variables|Hints|SetHint1_2 _returnvalue))))
  (UserInterface|Viewport|AddtoViewport _output_get 0))

(event Custom|MenuToOptions
  ;[1 1 1] Main Menu
  ;;[1 1 1] Menu to Options
  (Widget|RemovefromParent (Variables|Widgets|GetMainMenuWidget))
  (Utilities|IsValid (Variables|Widgets|GetMenuOptions)
    (:Is%20Valid
      _)
    (:Is%20Not%20Valid
      (bind _returnvalue (UserInterface|CreateWidget "/Game/UI/WB_MainMenuOptions.WB_MainMenuOptions_C" (Game|GetPlayerController 0)))
      (bind _output_get (Variables|Widgets|SetMenuOptions _returnvalue))))
  (UserInterface|Viewport|AddtoViewport _output_get 0))

(event Custom|OptionsToMenu
  ;[1 1 1] Main Menu
  ;;[1 1 1] Options to Menu
  (Widget|RemovefromParent (Variables|Widgets|GetMenuOptions))
  (UserInterface|Viewport|AddtoViewport (Variables|Widgets|GetMainMenuWidget) 0))

(event Custom|StartHint2_1
  ;[1 1 1] Hints
  ;;[1 1 1] Hints2
  (Utilities|IsValid (Variables|Hints|GetHint2_1)
    (:Is%20Valid
      _)
    (:Is%20Not%20Valid
      (bind _returnvalue (UserInterface|CreateWidget "/Game/UI/Hints/Hint2_1.Hint2_1_C"))
      (bind _output_get (Variables|Hints|SetHint2_1 _returnvalue))))
  (UserInterface|Viewport|AddtoViewport _output_get 0)
  (Input|SetInputModeUIOnly (Game|GetPlayerController 0) 0 "LockInFullscreen"))

(event Custom|StartHint2_2
  ;[1 1 1] Hints
  ;;[1 1 1] Hints2
  (Utilities|IsValid (Variables|Hints|GetHint2_2)
    (:Is%20Valid
      _)
    (:Is%20Not%20Valid
      (bind _returnvalue (UserInterface|CreateWidget "/Game/UI/Hints/Hint2_2.Hint2_2_C"))
      (bind _output_get (Variables|Hints|SetHint2_2 _returnvalue))))
  (UserInterface|Viewport|AddtoViewport _output_get 0))

(event Custom|PauseToOptions
  ;[1 1 1] Pause Menu
  ;;[1 1 1] Pause to Options
  (Widget|RemovefromParent (Variables|Widgets|GetPauseWidget))
  (Utilities|IsValid (Variables|Widgets|GetPauseOptions)
    (:Is%20Valid
      _)
    (:Is%20Not%20Valid
      (bind _returnvalue (UserInterface|CreateWidget "/Game/UI/WB_PauseMenuoptions.WB_PauseMenuOptions_C" (Game|GetPlayerController 0)))
      (bind _output_get (Variables|Widgets|SetPauseOptions _returnvalue))))
  (UserInterface|Viewport|AddtoViewport _output_get 0))

(event Custom|OptionsToPause
  ;[1 1 1] Pause Menu
  ;;[1 1 1] Options to Pause
  (Widget|RemovefromParent (Variables|Widgets|GetPauseOptions))
  (UserInterface|Viewport|AddtoViewport (Variables|Widgets|GetPauseWidget) 0))

(event Custom|StartHint2_3
  ;[1 1 1] Hints
  ;;[1 1 1] Hints2
  (Utilities|IsValid (Variables|Hints|GetHint2_3)
    (:Is%20Valid
      _)
    (:Is%20Not%20Valid
      (bind _returnvalue (UserInterface|CreateWidget "/Game/UI/Hints/Hint2_3.Hint2_3_C"))
      (bind _output_get (Variables|Hints|SetHint2_3 _returnvalue))))
  (UserInterface|Viewport|AddtoViewport _output_get 0))

(event Custom|BackToCheckpoint
  ;[1 1 1] Death Screen
  (Widget|RemovefromParent (Variables|Widgets|GetDeathScreenWidget))
  (bind _asbp_main_game_mode (Utilities|Casting|CastToBP_MainGameMode (Game|GetGameMode)))
  (if (Variables|/Script/WGAGame.WGAGameGameModeBase|GetbWasCheckpointReached _asbp_main_game_mode)
    (CallFunction|LoadCheckpoint)
    (else
      (CallFunction|DeathtoNewGame))))

(event Custom|StartHint2_4
  ;[1 1 1] Hints
  ;;[1 1 1] Hints2
  (Utilities|IsValid (Variables|Hints|GetHint2_4)
    (:Is%20Valid
      _)
    (:Is%20Not%20Valid
      (bind _returnvalue (UserInterface|CreateWidget "/Game/UI/Hints/Hint2_4.Hint2_4_C"))
      (bind _output_get (Variables|Hints|SetHint2_4 _returnvalue))))
  (UserInterface|Viewport|AddtoViewport _output_get 0))

(event Custom|StartHint2_5
  ;[1 1 1] Hints
  ;;[1 1 1] Hints2
  (Utilities|IsValid (Variables|Hints|GetHint2_5)
    (:Is%20Valid
      _)
    (:Is%20Not%20Valid
      (bind _returnvalue (UserInterface|CreateWidget "/Game/UI/Hints/Hint2_5.Hint2_5_C"))
      (bind _output_get (Variables|Hints|SetHint2_5 _returnvalue))))
  (UserInterface|Viewport|AddtoViewport _output_get 0))

(event Custom|StartHint3_1
  ;[1 1 1] Hints
  (Utilities|IsValid (Variables|Hints|GetHint3_1)
    (:Is%20Valid
      _)
    (:Is%20Not%20Valid
      (bind _returnvalue (UserInterface|CreateWidget "/Game/UI/Hints/Hint3_1.Hint3_1_C"))
      (bind _output_get (Variables|Hints|SetHint3_1 _returnvalue))))
  (UserInterface|Viewport|AddtoViewport _output_get 0)
  (Input|SetInputModeUIOnly (Game|GetPlayerController 0) 0 "LockInFullscreen"))

(event Custom|StartHint4_1
  ;[1 1 1] Hints
  (Utilities|IsValid (Variables|Hints|GetHint4_1)
    (:Is%20Valid
      _)
    (:Is%20Not%20Valid
      (bind _returnvalue (UserInterface|CreateWidget "/Game/UI/Hints/Hint4_1.Hint4_1_C"))
      (bind _output_get (Variables|Hints|SetHint4_1 _returnvalue))))
  (UserInterface|Viewport|AddtoViewport _output_get 0)
  (Input|SetInputModeUIOnly (Game|GetPlayerController 0) 0 "LockInFullscreen"))

(event Custom|StartHint5_1
  ;[1 1 1] Hints
  (Utilities|IsValid (Variables|Hints|GetHint5_1)
    (:Is%20Valid
      _)
    (:Is%20Not%20Valid
      (bind _returnvalue (UserInterface|CreateWidget "/Game/UI/Hints/Hint5_1.Hint5_1_C"))
      (bind _output_get (Variables|Hints|SetHint5_1 _returnvalue))))
  (UserInterface|Viewport|AddtoViewport _output_get 0)
  (Input|SetInputModeUIOnly (Game|GetPlayerController 0) 0 "LockInFullscreen"))

(event Custom|StartResult1
  ;[1 1 1] Hints
  ;;[1 1 1] Results
  (Utilities|IsValid (Variables|Results|GetResult1)
    (:Is%20Valid
      _)
    (:Is%20Not%20Valid
      (bind _returnvalue (UserInterface|CreateWidget "/Game/UI/Сonsequences/Result1.Result1_C"))
      (bind _output_get (Variables|Results|SetResult1 _returnvalue))))
  (UserInterface|Viewport|AddtoViewport _output_get 0)
  (Input|SetInputModeUIOnly (Game|GetPlayerController 0) 0 "LockInFullscreen"))

(event Custom|StartHint6_1
  ;[1 1 1] Hints
  (Utilities|IsValid (Variables|Hints|GetHint6_1)
    (:Is%20Valid
      _)
    (:Is%20Not%20Valid
      (bind _returnvalue (UserInterface|CreateWidget "/Game/UI/Hints/Hint6_1.Hint6_1_C"))
      (bind _output_get (Variables|Hints|SetHint6_1 _returnvalue))))
  (UserInterface|Viewport|AddtoViewport _output_get 0)
  (Input|SetInputModeUIOnly (Game|GetPlayerController 0) 0 "LockInFullscreen"))

(event Custom|StartResult2a
  ;[1 1 1] Hints
  ;;[1 1 1] Results
  (Utilities|IsValid (Variables|Results|GetResult2a)
    (:Is%20Valid
      _)
    (:Is%20Not%20Valid
      (bind _returnvalue (UserInterface|CreateWidget "/Game/UI/Сonsequences/Result2a.Result2a_C"))
      (bind _output_get (Variables|Results|SetResult2a _returnvalue))))
  (UserInterface|Viewport|AddtoViewport _output_get 0)
  (Input|SetInputModeUIOnly (Game|GetPlayerController 0) 0 "LockInFullscreen"))

(event Custom|StarResult2b
  ;[1 1 1] Hints
  ;;[1 1 1] Results
  (Utilities|IsValid (Variables|Results|GetResult2b)
    (:Is%20Valid
      _)
    (:Is%20Not%20Valid
      (bind _returnvalue (UserInterface|CreateWidget "/Game/UI/Сonsequences/Result2b.Result2b_C"))
      (bind _output_get (Variables|Results|SetResult2b _returnvalue))))
  (UserInterface|Viewport|AddtoViewport _output_get 0)
  (Input|SetInputModeUIOnly (Game|GetPlayerController 0) 0 "LockInFullscreen"))

(event Custom|TutorStart
  ;[1 1 1] Hints
  (Game|SetGamePaused true)
  (Utilities|IsValid (Variables|Hints|GetTutor)
    (:Is%20Valid
      _)
    (:Is%20Not%20Valid
      (bind _returnvalue (UserInterface|CreateWidget "/Game/UI/Hints/Tutorial.Tutorial_C"))
      (bind _output_get (Variables|Hints|SetTutor _returnvalue))))
  (UserInterface|Viewport|AddtoViewport _output_get 0)
  (Input|SetInputModeUIOnly (Game|GetPlayerController 0) 0 "LockInFullscreen"))

(event Custom|Start%20Game
  ;[1 1 1] Main Menu
  ;;[1 1 1] Начало Игры
  (Widget|RemovefromParent (Variables|Widgets|GetMainMenuWidget))
  (CallFunction|ShowLoadingScreen)
  (Utilities|FlowControl|Delay 2.0)
  (Game|OpenLevel(byName) "Level1_rebuild")
  (Input|SetInputModeGameandUI (Game|GetPlayerController 0) 0 "DoNotLock" true))

(event Custom|Show%20Pause%20Menu
  (bind _returnvalue (Game|GetPlayerController 0))
  ;[1 1 1] Pause Menu
  ;;[1 1 1] Show Pause Menu
  (Utilities|IsValid (Variables|Widgets|GetPauseWidget)
    (:Is%20Valid
      _)
    (:Is%20Not%20Valid
      (bind _returnvalue_2 (UserInterface|CreateWidget "/Game/UI/WB_PauseMenu.WB_PauseMenu_C" _returnvalue))
      (bind _output_get (Variables|Widgets|SetPauseWidget _returnvalue_2))))
  (UserInterface|Viewport|AddtoViewport _output_get 0)
  (Input|SetInputModeUIOnly _returnvalue (Variables|Widgets|GetPauseWidget) "LockInFullscreen")
  (Game|SetGamePaused true)
  (Variables|Logic|SetInPause true))

(event Custom|Resume%20Game
  ;[1 1 1] Pause Menu
  ;;[1 1 1] Resume Game
  (Widget|RemovefromParent (Variables|Widgets|GetPauseWidget))
  (Input|SetInputModeGameandUI (Game|GetPlayerController 0) 0 "DoNotLock" false)
  (Game|SetGamePaused false)
  (Variables|Logic|SetInPause false))

(event Custom|Pause%20to%20Menu
  ;[1 1 1] Pause Menu
  ;;[1 1 1] Back to Main Menu from Pause
  (Game|OpenLevel(byName) "MainMenu")
  (Variables|Logic|SetInPause false))

(event Custom|ShowDeathScreen
  (bind _returnvalue (Game|GetPlayerController 0))
  ;[1 1 1] Death Screen
  ;;[1 1 1] Show DeathScreen
  (Game|SetGamePaused true)
  (Utilities|IsValid (Variables|Widgets|GetDeathScreenWidget)
    (:Is%20Valid
      _)
    (:Is%20Not%20Valid
      (bind _returnvalue_2 (UserInterface|CreateWidget "/Game/UI/WB_DeathScreen.WB_DeathScreen_C" _returnvalue))
      (bind _output_get (Variables|Widgets|SetDeathScreenWidget _returnvalue_2))))
  (UserInterface|Viewport|AddtoViewport _output_get 0)
  (Input|SetInputModeUIOnly _returnvalue 0 "LockInFullscreen"))

(event Custom|LoadCheckpoint
  ;[1 1 1] Death Screen
  (Widget|RemovefromParent (Variables|Widgets|GetDeathScreenWidget))
  (bind _asbp_main_game_mode (Utilities|Casting|CastToBP_MainGameMode (Game|GetGameMode)))
  (Class|WGAGameGameModeBase|LoadCheckpoint _asbp_main_game_mode)
  (Input|SetInputModeGameandUI (Game|GetPlayerController 0) 0 "DoNotLock" true)
  (Game|SetGamePaused false))

(event Custom|OutOfHint
  ;[1 1 1] Hints
  ;;[1 1 1] OutOfHint
  (Game|SetGamePaused false)
  (Input|SetInputModeGameandUI (Game|GetPlayerController 0) 0 "DoNotLock" true))