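; BP_MainCharacter is a player character with cursor-facing, top-down style controls and a melee weapon.
; On BeginPlay it spawns BP_MeleeWeaponTest and attaches it to the mesh's WeaponSocket.
; Movement inputs push along fixed world axes scaled by MoveSpeed, while Tick yaws the capsule from a cursor trace with a 90-degree offset.
; Left Hand input raises the LeftHandAttack flag, then clears it after a short delay.
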(event EventBeginPlay
  ;[1 1 1] Spawn a weapon in character's hand
  (bind _returnvalue (Game|SpawnActorfromClass "/Game/Weapon/BP_MeleeWeaponTest.BP_MeleeWeaponTest_C" (Transformation|GetSocketTransform (Variables|Character|GetMesh) "WeaponSocket" "RTS_World") "Undefined" 0 0))
  (Transformation|AttachComponentToComponent _returnvalue (Variables|Character|GetMesh) "WeaponSocket" "KeepRelative" "KeepRelative" "KeepRelative" true))

(event EventTick
  (params (DeltaSeconds :type Float%20%28single-precision%29))
  (bind _returnvalue (Game|GetPlayerController 0))
  (bind _returnvalue_2 (Transformation|GetActorLocation))
  (bind _hitresult (Game|Player|GetHitResultUnderCursorbyChannel _returnvalue "TraceTypeQuery1" true))
  (bind _returnvalue_3 (- _returnvalue_2 (.location _hitresult)))
  ;[1 1 1] Rotation to mouse
  (Transformation|SetWorldRotation (Variables|Collision|GetCapsuleComponent) (Math|Rotator|MakeRotator 0.0 0.0 (+ (.yaw (Math|Rotator|MakeRotationfromAxes (Math|Vector|MakeVector (.x _returnvalue_3) (.y _returnvalue_3) 0.0) "0, 0, 0" "0, 0, 0")) 9e+01)) false false))

(event Input|ActionEvents|InputActionLeftHand
  (params (Key :type Key%20Structure :default "None"))
  (:Pressed
    (Variables|Default|SetLeft_Hand_Attack true)
    (Utilities|FlowControl|Delay 1.0)
    (Variables|Default|SetLeft_Hand_Attack false)))

(event Input|AxisEvents|InputAxisMoveRight
  (params (AxisValue :type Float%20%28single-precision%29))
  ;[1 1 1] Movement
  (Pawn|Input|AddMovementInput "0.000000,1.000000,0.000000" (* AxisValue (Variables|Default|GetMoveSpeed)) false))

(event Input|AxisEvents|InputAxisMoveForward
  (params (AxisValue :type Float%20%28single-precision%29))
  ;[1 1 1] Movement
  (Pawn|Input|AddMovementInput "1.000000,0.000000, 0" (* AxisValue (Variables|Default|GetMoveSpeed)) false))

(fn ConstructionScript)